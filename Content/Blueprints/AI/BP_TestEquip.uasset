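; BP_TestEquip is a test Blueprint for equipping armor picked up from the world.
; On BeginPlay it casts itself to PlayerController and adds the BTS and TestEquip Enhanced Input mapping contexts.
; IA_Equip scans actors overlapping the player character for the "Armor" tag, copies the BP_Armor static mesh onto BP_TextAIPlayer's Armor component, destroys the pickup and prints a display name.
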(event Input|EnhancedActionEvents|EnhancedInputActionIA_Equip
  (params (ActionValue :type Boolean) (ElapsedSeconds :type Float%20%28double-precision%29) (TriggeredSeconds :type Float%20%28double-precision%29) (InputAction :type Input%20Action%20Object%20Reference :default "/Game/Blueprints/AI/IA_Equip.IA_Equip"))
  (for _array_element (Collision|GetOverlappingActors (Game|GetPlayerCharacter 0) "/Script/Engine.Actor" :!class /Script/Engine.Actor)
    (if (Actor|ActorHasTag _array_element "Armor")
      (bind _asbp_armor (Utilities|Casting|CastToBP_Armor _array_element))
      (bind _asbp_text_aiplayer (Utilities|Casting|CastToBP_TextAIPlayer (Game|GetPlayerCharacter 0)))
      (Components|StaticMesh|SetStaticMesh (Variables|/Game/Blueprints/AI/BP_TextAIPlayer.BP_TextAIPlayer_C|GetArmor _asbp_text_aiplayer) (Variables|/Script/Engine.StaticMeshComponent|GetStaticMesh (Variables|/Game/Blueprints/AI/BP_Armor.BP_Armor_C|GetStaticMesh _asbp_armor)))
      (Actor|DestroyActor _asbp_armor)
      (Development|PrintString (Utilities|GetDisplayName 0)))))

(event EventBeginPlay
  (bind _as플레이어_컨트롤러 (Utilities|Casting|CastToPlayerController self))
  (Utilities|IsValid _as플레이어_컨트롤러
    (:Is%20Valid
      (Input|AddMappingContext (PlayerController|LocalPlayerSubsystems|GetEnhancedInputLocalPlayerSubsystem _as플레이어_컨트롤러) "/Game/Blueprints/Input/IMC_BTSInputContext.IMC_BTSInputContext" 0 "(bIgnoreAllPressedKeysUntilRelease=True,bForceImmediately=False,bNotifyUserSettings=False)")
      (Input|AddMappingContext (PlayerController|LocalPlayerSubsystems|GetEnhancedInputLocalPlayerSubsystem _as플레이어_컨트롤러) "/Game/Blueprints/AI/IMC_TestEquip.IMC_TestEquip" 0 "(bIgnoreAllPressedKeysUntilRelease=True,bForceImmediately=False,bNotifyUserSettings=False)"))))

(event EventTick
  (params (DeltaSeconds :type Float%20%28single-precision%29)))

(fn ConstructionScript)