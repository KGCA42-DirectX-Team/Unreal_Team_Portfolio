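; BP_TextAIPlayer is a player character in the AI folder that launches noise test actors, apparently for AI testing.
; Despite its name, the ChangePerspective event spawns a BP_NoiseTestActor just ahead of the capsule and sets its projectile velocity along the forward vector.
; A FlipFlop switching first- and third-person cameras and orient-rotation-to-movement remains in the graph but is disconnected and never runs.
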(event EventBeginPlay)

(event Collision|EventActorBeginOverlap
  (params (OtherActor :type Actor%20Object%20Reference)))

(event EventTick
  (params (DeltaSeconds :type Float%20%28single-precision%29)))

(event EventChangePerspective
  (bind _returnvalue (Game|SpawnActorfromClass "/Game/Blueprints/AI/BP_NoiseTestActor.BP_NoiseTestActor_C" (Math|Conversions|ToTransform(Vector) (+ (Transformation|GetActorLocation) (* (Math|Vector|GetForwardVector (Variables|Default|GetCapsuleComponent)) 2e+01))) "Undefined" "MultiplyWithRoot" 0 0))
  (Variables|/Script/Engine.MovementComponent|SetVelocity (Variables|/Game/Blueprints/AI/BP_NoiseTestActor.BP_NoiseTestActor_C|GetProjectileMovement _returnvalue) (* (Math|Vector|GetForwardVector (Variables|Default|GetCapsuleComponent)) 1e+03)))

(fn ConstructionScript)