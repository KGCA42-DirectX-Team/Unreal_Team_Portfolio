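; Test enemy AI Blueprint, named as deprecated, with limb dismemberment and a Runaway flag written to its Blackboard every Tick.
; AnyDamage maps child bones to their limb or spine root, then subtracts damage from that bone's entry in a durability map.
; At zero durability the bone is hidden, and arms and legs spawn a severed-limb actor at the socket, with BrokenBones guarding against repeat spawns.
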(event EventBeginPlay)

(event Collision|EventActorBeginOverlap
  (params (OtherActor :type Actor%20Object%20Reference)))

(event EventTick
  (params (DeltaSeconds :type Float%20%28single-precision%29))
  (AI|Components|Blackboard|SetValueasBool (AI|GetBlackboard 0) (Variables|Default|GetKey%20Name) (Variables|Default|GetRunaway)))

(fn ConstructionScript)

(fn GetAnimationState
  (return "Unarmed"))

(fn AnyDamage
  (params (Damage :type Float%20%28double-precision%29) (HitBoneName :type Name) (DamageCauser :type Actor%20Object%20Reference))
  (Variables|Default|SetAppliedDamage Damage)
  (Variables|Default|SetHitBoneName HitBoneName)
  (Variables|Default|SetDamage%20Causer DamageCauser)
  (CallFunction|RenameBoneName)
  (bind _reacheddurabilitylimit (CallFunction|ApplyDamagetoBone))
  (if _reacheddurabilitylimit
    (CallFunction|Dismemberment)))

(fn RenameBoneName
  (switch name (Variables|Default|GetHitBoneName)
    (:spine_02
      (Variables|Default|SetHitBoneName "Spine_01" :!label _label))
    (:spine_03
      (goto _label))
    (:lowerarm_l
      (Variables|Default|SetHitBoneName "upperarm_l" :!label _label_2))
    (:hand_l
      (goto _label_2))
    (:lowerarm_r
      (Variables|Default|SetHitBoneName "upperarm_r" :!label _label_3))
    (:hand_r
      (goto _label_3))
    (:calf_l
      (Variables|Default|SetHitBoneName "thigh_l" :!label _label_4))
    (:foot_l
      (goto _label_4))
    (:calf_r
      (Variables|Default|SetHitBoneName "thigh_r" :!label _label_5))
    (:foot_r
      (goto _label_5))))

(fn ApplyDamagetoBone
  (bind _breakablebones_bonedurability (Variables|Default|GetBreakableBones/BoneDurability))
  (bind _hitbonename (Variables|Default|GetHitBoneName))
  (bind (_value _returnvalue) (Utilities|Map|Find _breakablebones_bonedurability _hitbonename))
  (if _returnvalue
    (Utilities|Map|Add (Variables|Default|GetBreakableBones/BoneDurability) (Variables|Default|GetHitBoneName) (- _value (Variables|Default|GetAppliedDamage)))
    (return (<= (.Value (Utilities|Map|Find (Variables|Default|GetBreakableBones/BoneDurability) (Variables|Default|GetHitBoneName))) 0.0))))

(fn Dismemberment
  (bind _hitbonename (Variables|Default|GetHitBoneName))
  (Components|SkinnedMesh|HideBonebyName (Variables|Character|GetMesh) _hitbonename "PBO_None")
  (switch name _hitbonename
    (:thigh_l
      (Variables|Default|SetDismemberClass "/Game/Blueprints/Dismember/BP_Leg_l.BP_Leg_l_C"))
    (:thigh_r
      (Variables|Default|SetDismemberClass "/Game/Blueprints/Dismember/BP_Leg_R.BP_Leg_R_C"))
    (:upperarm_l
      (Variables|Default|SetDismemberClass "/Game/Blueprints/Dismember/BP_Arm_l.BP_Arm_l_C"))
    (:upperarm_r
      (Variables|Default|SetDismemberClass "/Game/Blueprints/Dismember/BP_Arm_R.BP_Arm_R_C")))
  (for _array_element (Variables|Default|GetBrokenBones)
    (if (== _array_element (Variables|Default|GetHitBoneName))
      (LocalVariables|SetIsBrokenBone (== _array_element (Variables|Default|GetHitBoneName)))))
  (if (not (LocalVariables|GetIsBrokenBone))
    (Game|SpawnActorfromClass (Variables|Default|GetDismemberClass) (Transformation|GetSocketTransform (Variables|Character|GetMesh) _hitbonename "RTS_World") "Undefined" "MultiplyWithRoot" 0 0)
    (Utilities|Array|Add (Variables|Default|GetBrokenBones) (Variables|Default|GetHitBoneName))))