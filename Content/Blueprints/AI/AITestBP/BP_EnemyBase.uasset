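; Base enemy AI character that equips weapons, evades grenades and supports limb dismemberment.
; BeginPlay adds weapon and inventory components and binds events that wield the weapon or write grenade evasion keys to the Blackboard.
; AnyDamage remaps hit bones to parent limbs or lower spine, then subtracts damage from per-bone durability.
; Depleted bones are hidden, with a one-time limb spawn for thighs and upper arms, though its classes are unset here.
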(event Custom|EquipWeapon
  (bind _asbp_weapon_component (Utilities|Casting|CastToBP_WeaponComponent (Variables|Default|GetWeaponComponent)))
  (Default|WieldWeapon _asbp_weapon_component))

(event Custom|EvadeFromGranade
  (params (Granade :type Actor%20Object%20Reference))
  (bind _returnvalue (AI|GetBlackboard 0))
  (AI|Components|Blackboard|SetValueasObject _returnvalue (Utilities|Name|MakeLiteralName "GranadeActor") Granade)
  (AI|Components|Blackboard|SetValueasBool _returnvalue (Utilities|Name|MakeLiteralName "EvadeGranade") true))

(event EventBeginPlay
  (bind _returnvalue (AddComponent|AddBPWeaponComponent))
  (Variables|Default|SetWeaponComponent _returnvalue)
  (bind _returnvalue_2 (AddComponent|AddBPInventoryComponent 0 0 false))
  (Variables|Default|SetInventoryComponent _returnvalue_2)
  (EventDispatchers|BindEventtoEquipWeaponEvent (delegate Custom|EquipWeapon))
  (EventDispatchers|BindEventtoEvadeGranade (delegate Custom|EvadeFromGranade)))

(event Collision|EventActorBeginOverlap
  (params (OtherActor :type Actor%20Object%20Reference)))

(event EventSetAnimationState
  (params (NewState :type EAnimationState%20Enum :default "None"))
  (Variables|Default|SetAnimationState NewState))

(event Game|Damage|EventRadialDamage
  (params (DamageReceived :type Float%20%28single-precision%29) (DamageType :type Damage%20Type%20Object%20Reference) (Origin :type Vector :default "0, 0, 0") (HitInfo :type Hit%20Result%20Structure%20%28by%20ref%29) (InstigatedBy :type Controller%20Object%20Reference) (DamageCauser :type Actor%20Object%20Reference))
  (Variables|Default|SetImpactNormal (.ImpactNormal (Collision|BreakHitResult HitInfo))))

(fn ConstructionScript)

(fn GetAnimationState
  (return (Variables|Default|GetAnimationState)))

(fn Dismemberment
  (bind _hitbonename (Variables|Default|GetHitBoneName))
  (Components|SkinnedMesh|HideBonebyName (Variables|Character|GetMesh) _hitbonename "PBO_None")
  (switch name _hitbonename
    (:thigh_l
      (Variables|Default|SetDismemberClass 0))
    (:thigh_r
      (Variables|Default|SetDismemberClass 0))
    (:upperarm_l
      (Variables|Default|SetDismemberClass 0))
    (:upperarm_r
      (Variables|Default|SetDismemberClass 0)))
  (for _array_element (Variables|Default|GetBrokenBones)
    (if (== _array_element (Variables|Default|GetHitBoneName))
      (Variables|Default|SetIsBrokenBone (== _array_element (Variables|Default|GetHitBoneName)))))
  (if (not (Variables|Default|GetIsBrokenBone))
    (Game|SpawnActorfromClass (Variables|Default|GetDismemberClass) (Transformation|GetSocketTransform (Variables|Character|GetMesh) _hitbonename "RTS_World") "Undefined" "MultiplyWithRoot" 0 0)
    (Utilities|Array|Add (Variables|Default|GetBrokenBones) (Variables|Default|GetHitBoneName))))

(fn ApplyDamagetoBone
  (bind _breakablebones_bonedurability (Variables|Default|GetBreakableBones/BoneDurability))
  (bind _hitbonename (Variables|Default|GetHitBoneName))
  (bind (_value _returnvalue) (Utilities|Map|Find _breakablebones_bonedurability _hitbonename))
  (if _returnvalue
    (Utilities|Map|Add (Variables|Default|GetBreakableBones/BoneDurability) (Variables|Default|GetHitBoneName) (- _value (Variables|Default|GetAppliedDamage)))
    (return (<= (.Value (Utilities|Map|Find (Variables|Default|GetBreakableBones/BoneDurability) (Variables|Default|GetHitBoneName))) 0.0))))

(fn RenameBoneName
  (switch name (Variables|Default|GetHitBoneName)
    (:spine_02
      (Variables|Default|SetHitBoneName "Spine_01" :!label _label))
    (:spine_03
      (goto _label))
    (:lowerarm_l
      (Variables|Default|SetHitBoneName "upperarm_l" :!label _label_2))
    (:hand_l
      (goto _label_2))
    (:lowerarm_r
      (Variables|Default|SetHitBoneName "upperarm_r" :!label _label_3))
    (:hand_r
      (goto _label_3))
    (:calf_l
      (Variables|Default|SetHitBoneName "thigh_l" :!label _label_4))
    (:foot_l
      (goto _label_4))
    (:calf_r
      (Variables|Default|SetHitBoneName "thigh_r" :!label _label_5))
    (:foot_r
      (goto _label_5))))

(fn AnyDamage
  (params (NewParam :type Float%20%28double-precision%29) (NewParam1 :type Name) (NewParam2 :type Actor%20Object%20Reference))
  (Variables|Default|SetAppliedDamage NewParam)
  (Variables|Default|SetHitBoneName NewParam1)
  (Variables|Default|SetDamage%20Causer NewParam2)
  (CallFunction|RenameBoneName)
  (bind _reacheddurabilitylimit (CallFunction|ApplyDamagetoBone))
  (if _reacheddurabilitylimit
    (CallFunction|Dismemberment)))