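; BP_NoiseTestActor is an AI test actor that makes a noise when its static mesh registers a hit.
; On the first hit only, gated by a DoOnce with no reset, it reports an AI hearing noise event and plays a camera shutter sound at the impact point.
; If the other actor has an Ability System Component, that component applies the configured GameplayEffectClass to itself.
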(event OnComponentHit(StaticMesh)
  (params (HitComponent :type Primitive%20Component%20Object%20Reference) (OtherActor :type Actor%20Object%20Reference) (OtherComp :type Primitive%20Component%20Object%20Reference) (NormalImpulse :type Vector :default "0, 0, 0") (Hit :type Hit%20Result%20Structure%20%28by%20ref%29))
  (bind _location (Collision|BreakHitResult Hit))
  (bind _returnvalue (Ability|GetAbilitySystemComponent OtherActor))
  (Utilities|FlowControl|DoOnce false
    (:Completed
      (Class|AISenseHearing|ReportNoiseEvent _location 2.0 self 1e+03 "None")
      (Audio|SpawnSoundatLocation "/Engine/VREditor/Sounds/UI/Camera_Shutter.Camera_Shutter" _location "0, 0, 0" 1.0 1.0 0.0 0 0)
      (Utilities|IsValid _returnvalue
        (:Is%20Valid
          (GameplayEffects|ApplyGameplayEffectSpecToSelf _returnvalue (GameplayEffects|MakeOutgoingSpec _returnvalue (Variables|Default|GetGameplay%20Effect%20Class) 0.0 (GameplayEffects|MakeEffectContext _returnvalue))))))))

(event EventBeginPlay)

(event Collision|EventActorBeginOverlap
  (params (OtherActor :type Actor%20Object%20Reference)))

(event EventTick
  (params (DeltaSeconds :type Float%20%28single-precision%29)))

(fn ConstructionScript)