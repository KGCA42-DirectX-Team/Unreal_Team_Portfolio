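; Test player character for AI work, with camera-trace damage on BP_Enemy, interface-based interaction, an inventory widget and first/third-person camera switching.
; Tick traces for interactables and applies parachute physics, overriding gravity, air control and fall velocity.
; Landing classifies impact speed and hides the parachute; debug keys switch weapon animation states.
; Trace-based mantling with motion warping is implemented, but its calling chain is disconnected.
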(event Custom|InventoryTempInput
  (bind _returnvalue (Game|GetPlayerController 0))
  (bind _returnvalue_2 (Game|GetPlayerController 0))
  (bind _inventorywidget (Variables|Default|GetInventoryWidget))
  (if (UserInterface|Viewport|IsinViewport _inventorywidget)
    (Widget|RemovefromParent _inventorywidget)
    (Input|SetInputModeGameOnly _returnvalue_2 false)
    (Variables|/Script/Engine.PlayerController|SetbShowMouseCursor _returnvalue_2 false)
    (else
      (UserInterface|Viewport|AddtoViewport _inventorywidget 0)
      (Input|SetInputModeGameandUI _returnvalue (Variables|Default|GetInventoryWidget) "DoNotLock" false false)
      (Variables|/Script/Engine.PlayerController|SetbShowMouseCursor _returnvalue true))))

(event EventBeginPlay
  (Input|EnableInput (Game|GetPlayerController 0))
  (Variables|Components|SetCharacterMesh (Variables|Character|GetMesh))
  (Variables|Default|SetAnimationState "Unarmed")
  (bind _returnvalue (UserInterface|CreateWidget "/Game/Blueprints/UI/InventoryWidget/WBP_InventoryWidget.WBP_InventoryWidget_C" (Game|GetPlayerController 0) (Variables|Default|GetInventoryComponent) 5e+01))
  (Variables|Default|SetInventoryWidget _returnvalue)
  (bind _asbp_parachute (Utilities|Casting|CastToBP_Parachute (Variables|/Script/Engine.ChildActorComponent|GetChildActor (Variables|Default|GetBP_Parachute))))
  (Variables|Default|SetBP%20Parachute _asbp_parachute))

(event EventTick
  (params (DeltaSeconds :type Float%20%28single-precision%29))
  (Utilities|FlowControl|Sequence
    (:then_0
      (CallFunction|LineTraceTTP))
    (:then_1
      (CallFunction|SetGravityandAir))))

(event EventChangePerspective
  (bind _charactermovement (Variables|Character|GetCharacterMovement))
  (Utilities|FlowControl|FlipFlop
    (:A
      (Components|Activation|SetActive (Variables|Components|GetFPP_Camera) true false)
      (Components|Activation|SetActive (Variables|Components|GetTTP_Camera) false false)
      (Variables|/Script/Engine.CharacterMovementComponent|SetbOrientRotationToMovement _charactermovement true))
    (:B
      (Components|Activation|SetActive (Variables|Components|GetFPP_Camera) false false)
      (Components|Activation|SetActive (Variables|Components|GetTTP_Camera) true false)
      (Variables|/Script/Engine.CharacterMovementComponent|SetbOrientRotationToMovement _charactermovement false))))

(event EventOnLanded
  (params (Hit :type Hit%20Result%20Structure%20%28by%20ref%29))
  (bind _charactermovement (Variables|Character|GetCharacterMovement))
  (bind _velocity (Variables|/Script/Engine.MovementComponent|GetVelocity _charactermovement))
  (bind _returnvalue (Math|Float|Absolute(Float) (.z _velocity)))
  (Utilities|FlowControl|Sequence
    (:then_0
      (if (Math|Float|InRange(Float) _returnvalue 3e+02 7.5e+02)
        (Variables|Default|SetOnLandState "NormalLand")))
    (:then_1
      (if (Math|Float|InRange(Float) _returnvalue 7.5e+02 1e+03)
        (Variables|Default|SetOnLandState "SoftLand")))
    (:then_2
      (if (> _returnvalue 1e+03)
        (Variables|Default|SetOnLandState "HardLand")))
    (:then_3
      (Variables|Default|SetSetParachute false)
      (Utilities|FlowControl|DoOnce false
        (:Completed
          (Rendering|SetVisibility (Variables|Default|GetBP_Parachute) false false)
          (Animation|PlayAnimMontage "/Game/Asset/parachute/AM_DiveRoll.AM_DiveRoll" 1.0 "None"))))))

(event Input|MouseEvents|LeftMouseButton
  (params (Key :type Key%20Structure :default "None"))
  (bind _fpp_camera (Variables|Components|GetFPP_Camera))
  (bind _returnvalue (Transformation|GetWorldLocation _fpp_camera))
  (:Pressed
    (bind _outhit (Collision|LineTraceByChannel _returnvalue (+ _returnvalue (* (Math|Vector|GetForwardVector (Transformation|GetWorldRotation _fpp_camera)) 1e+03)) "TraceTypeQuery1" true 0 "ForDuration" true "(R=1.000000,G=0.000000,B=0.000000,A=1.000000)" "(R=0.000000,G=1.000000,B=0.000000,A=1.000000)" 1.0))
    (bind _asbp_enemy (Utilities|Casting|CastToBP_Enemy (.HitActor (Collision|BreakHitResult _outhit))))
    (Default|AnyDamage _asbp_enemy 5.0 (.HitBoneName (Collision|BreakHitResult _outhit)) self)))

(event Input|KeyboardEvents|R
  (params (Key :type Key%20Structure :default "None"))
  (:Pressed
    (Animation|PlayAnimMontage "/Game/Asset/parachute/AM_DiveRoll.AM_DiveRoll" 1.0 "None")))

(event Input|KeyboardEvents|Z
  (params (Key :type Key%20Structure :default "None"))
  (:Pressed
    (if (not (Variables|Default|GetSetParachute))
      (if (AI|Components|NavMovement|IsFalling (Variables|Character|GetCharacterMovement))
        (Utilities|FlowControl|DoOnce false
          (:Completed
            (Variables|Default|SetSetParachute true)
            (Rendering|SetVisibility (Variables|Default|GetBP_Parachute) true false)))))))

(event Input|KeyboardEvents|F
  (params (Key :type Key%20Structure :default "None"))
  (bind _interactable_actor (Variables|Default|GetInteractable%20Actor))
  (bind _interactable_actor_2 (Variables|Default|GetInteractable%20Actor))
  (:Pressed
    (Utilities|IsValid _interactable_actor
      (:Is%20Valid
        (Class|BTSInteractionInterface|Interaction(Message) _interactable_actor))))
  (:Released
    (Utilities|IsValid _interactable_actor_2
      (:Is%20Valid
        (Class|BTSInteractionInterface|InteractionClear(Message) _interactable_actor_2)))))

(event Input|KeyboardEvents|7
  (params (Key :type Key%20Structure :default "None"))
  ;[1 1 1] Temp Anim State Change
  (:Pressed
    (Variables|Default|SetAnimationState "Unarmed")))

(event Input|KeyboardEvents|8
  (params (Key :type Key%20Structure :default "None"))
  ;[1 1 1] Temp Anim State Change
  (:Pressed
    (Variables|Default|SetAnimationState "Pistol")))

(event Input|KeyboardEvents|9
  (params (Key :type Key%20Structure :default "None"))
  ;[1 1 1] Temp Anim State Change
  (:Pressed
    (Variables|Default|SetAnimationState "Rifle")))

(fn ConstructionScript)

(fn MantleTrace
  (params (InitialTraceLength :type Float%20%28double-precision%29) (SecondaryTraceZOffset :type Float%20%28double-precision%29) (FallingHeightMultiplier :type Float%20%28double-precision%29))
  (bind _returnvalue (Transformation|GetActorLocation))
  ;[1 1 1] Trace for check object
  (Variables|Default|SetCanMantle false)
  (bind (_outhit _returnvalue_2) (Collision|LineTraceByChannel _returnvalue (+ _returnvalue (* (Transformation|GetActorForwardVector) InitialTraceLength)) "TraceTypeQuery1" false 0 "ForDuration"))
  ;[1 1 1] If an object is found tnen trace for ther object height. if player is falling then the maximum reachable height is lowered
  (if _returnvalue_2
    (bind (_outhit_2 _returnvalue_3) (Collision|SphereTraceByChannel (+ (.Location (Collision|BreakHitResult _outhit)) (Math|Vector|MakeVector 0.0 0.0 (* SecondaryTraceZOffset (Math|Float|SelectFloat FallingHeightMultiplier 1.0 (AI|Components|NavMovement|IsFalling (Variables|Character|GetCharacterMovement)))))) (.Location (Collision|BreakHitResult _outhit)) 1e+01 "TraceTypeQuery1" false 0 "ForDuration"))
    ;[1 1 1] Find the position to motion wap to using the detected points from the trace
    (if _returnvalue_3
      (LocalVariables|SetMantlePos1 (+ (.ImpactPoint (Collision|BreakHitResult _outhit_2)) (* (Transformation|GetActorForwardVector) -5e+01)))
      (bind _output_get (LocalVariables|SetMantlePos2 (+ (.ImpactPoint (Collision|BreakHitResult _outhit_2)) (* (Transformation|GetActorForwardVector) 1.2e+02))))
      ;[1 1 1] Do sphere trace to check if the player has enough space to land at the target location once
      (Variables|Default|SetCanMantle true)
      (bind _returnvalue_4 (Collision|SphereTraceByChannel (+ _output_get "0.000000,0.000000,20.000000") (+ _output_get "0.000000,0.000000,20.000000") 1e+01 "TraceTypeQuery1" false 0 "ForDuration"))
      (if _returnvalue_4
        (Variables|Default|SetCanMantle false)
        (else
          (LocalVariables|SetMantlePos2 (+ (.ImpactPoint (Collision|BreakHitResult _outhit_2)) (* (Transformation|GetActorForwardVector) 5e+01)))))
      ;[1 1 1] Do final trace to check if the path from the first and second mantle position is clear
      (if (or (Utilities|Operators|EqualEqual :A (LocalVariables|GetMantlePos1)) (Utilities|Operators|EqualEqual :A (LocalVariables|GetMantlePos2)))
        (Variables|Default|SetCanMantle false :!label _label)
        (else
          (bind _returnvalue_5 (Collision|SphereTraceByChannel (Math|Vector|MakeVector (.x (LocalVariables|GetMantlePos1)) (.y (LocalVariables|GetMantlePos1)) (.Z (Math|Vector|BreakVector (+ (LocalVariables|GetMantlePos2) "0.000000,0.000000,100.000000")))) (+ (LocalVariables|GetMantlePos2) "0.000000,0.000000,100.000000") 2e+01 "TraceTypeQuery1" false 0 "ForDuration"))
          (if _returnvalue_5
            (goto _label)
            (else
              _))))
      (return (LocalVariables|GetMantlePos1) (LocalVariables|GetMantlePos2)))
    (else
      (Variables|Default|SetCanMantle false))))

(fn GetPlayerController
  (bind _as플레이어_컨트롤러 (Utilities|Casting|CastToPlayerController (Pawn|GetController)))
  (return _as플레이어_컨트롤러))

(fn LineTraceTTP
  (bind _fpp_camera (Variables|Components|GetFPP_Camera))
  (bind _returnvalue (Transformation|GetWorldLocation _fpp_camera))
  (bind (_outhit _returnvalue_2) (Collision|LineTraceByChannel _returnvalue (+ _returnvalue (* (Math|Vector|GetForwardVector (Transformation|GetWorldRotation _fpp_camera)) 2e+02)) "TraceTypeQuery4" true 0 "ForDuration" true "(R=1.000000,G=0.000000,B=0.000000,A=1.000000)" "(R=0.000000,G=1.000000,B=0.000000,A=1.000000)" 1.0))
  (if _returnvalue_2
    (if (Utilities|DoesObjectImplementInterface (.HitActor (Collision|BreakHitResult _outhit)) "/Script/BrutalTakedownSquad.BTS_InteractionInterface")
      (Class|BTSInteractionInterface|Visible(Message) (.HitActor (Collision|BreakHitResult _outhit)))
      (Variables|Default|SetInteractable%20Actor (.HitActor (Collision|BreakHitResult _outhit))))
    (else
      (Utilities|IsValid (Variables|Default|GetInteractable%20Actor)
        (:Is%20Valid
          (Class|BTSInteractionInterface|InteractionClear(Message) (Variables|Default|GetInteractable%20Actor))
          (Variables|Default|SetInteractable%20Actor 0))))))

(fn SetGravityandAir
  (bind _returnvalue (Transformation|GetVelocity))
  (bind _setparachute (Variables|Default|GetSetParachute))
  (bind _charactermovement (Variables|Character|GetCharacterMovement))
  (bind _charactermovement_2 (Variables|Character|GetCharacterMovement))
  (bind (_x _y) (Math|Vector|BreakVector _returnvalue))
  (Default|SetParachuteVisible (Variables|Default|GetBP%20Parachute) _setparachute)
  (if _setparachute
    (Variables|/Script/Engine.CharacterMovementComponent|SetAirControl _charactermovement_2 2e+02)
    (Variables|/Script/Engine.CharacterMovementComponent|SetGravityScale _charactermovement_2 0.5)
    (Variables|/Script/Engine.MovementComponent|SetVelocity _charactermovement_2 (Math|Vector|MakeVector _x _y -3e+02))
    (else
      (Variables|/Script/Engine.CharacterMovementComponent|SetAirControl _charactermovement 0.2)
      (Variables|/Script/Engine.CharacterMovementComponent|SetGravityScale _charactermovement 1.0))))