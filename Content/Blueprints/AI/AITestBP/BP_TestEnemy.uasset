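; Test enemy AI character with per-bone dismemberment, built from modular male body meshes that follow the main mesh's pose.
; AnyDamage remaps pelvis and upper-spine hits to spine_02, then subtracts damage from that bone's durability in a map.
; Depleted bones have their physics constraint broken and are recorded, with a flag for whether it was the spine.
; Tick copies the Runaway flag to the Blackboard, and animation state is always Unarmed.
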(event EventBeginPlay)

(event Collision|EventActorBeginOverlap
  (params (OtherActor :type Actor%20Object%20Reference)))

(event EventTick
  (params (DeltaSeconds :type Float%20%28single-precision%29))
  (AI|Components|Blackboard|SetValueasBool (AI|GetBlackboard 0) (Variables|Default|GetKey%20Name) (Variables|Default|GetRunaway)))

(fn ConstructionScript
  (Components|SkinnedMesh|SetLeaderPoseComponent (Variables|Default|GetMW_Style2_Male_leg_R) (Variables|Character|GetMesh) false false))

(fn GetAnimationState
  (return "Unarmed"))

(fn AnyDamage
  (params (Damage :type Float%20%28double-precision%29) (HitBoneName :type Name) (DamageCauser :type Actor%20Object%20Reference))
  (Variables|Default|SetAppliedDamage Damage)
  (Variables|Default|SetHitBoneName HitBoneName)
  (Variables|Default|SetDamage%20Causer DamageCauser)
  (CallFunction|RenameBoneName)
  (bind _reacheddurabilitylimit (CallFunction|ApplyDamagetoBone))
  (if _reacheddurabilitylimit
    (CallFunction|Dismemberment)))

(fn RenameBoneName
  (switch name (Variables|Default|GetHitBoneName)
    (:pelvis
      _)
    (:spine_05
      _)
    (:spine_04
      _))
  (Variables|Default|SetHitBoneName "spine_02"))

(fn ApplyDamagetoBone
  (bind _breakablebones_bonedurability (Variables|Default|GetBreakableBones/BoneDurability))
  (bind _hitbonename (Variables|Default|GetHitBoneName))
  (bind (_value _returnvalue) (Utilities|Map|Find _breakablebones_bonedurability _hitbonename))
  (if _returnvalue
    (Utilities|Map|Add (Variables|Default|GetBreakableBones/BoneDurability) (Variables|Default|GetHitBoneName) (- _value (Variables|Default|GetAppliedDamage)))
    (return (<= (.Value (Utilities|Map|Find (Variables|Default|GetBreakableBones/BoneDurability) (Variables|Default|GetHitBoneName))) 0.0))))

(fn Dismemberment
  (bind _hitbonename (Variables|Default|GetHitBoneName))
  (Class|SkeletalMeshComponent|BreakConstraint (Variables|Character|GetMesh) "0, 0, 0" "0, 0, 0" _hitbonename)
  (Variables|Default|SetHasSpineBroken (== _hitbonename "spine_02"))
  (Utilities|Array|Add (Variables|Default|GetBrokenBones) (Variables|Default|GetHitBoneName)))