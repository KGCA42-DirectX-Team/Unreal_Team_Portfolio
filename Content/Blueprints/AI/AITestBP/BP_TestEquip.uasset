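; Test Blueprint for equipping armor through Enhanced Input, with the equip logic currently disconnected.
; BeginPlay casts itself to PlayerController and adds the default character and TestEquip mapping contexts.
; The IA_Equip event is empty.
; An unreachable chain searches the player's overlapping actors for the Armor tag, copies that BP_Armor's mesh onto BP_TestPlayer's Armor component, then destroys the pickup.
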(event Input|EnhancedActionEvents|EnhancedInputActionIA_Equip
  (params (ActionValue :type Boolean) (ElapsedSeconds :type Float%20%28double-precision%29) (TriggeredSeconds :type Float%20%28double-precision%29) (InputAction :type Input%20Action%20Object%20Reference :default "/Game/Blueprints/AI/AITestBP/IA_Equip.IA_Equip")))

(event EventBeginPlay
  (bind _asplayer_controller (Utilities|Casting|CastToPlayerController self))
  (Utilities|IsValid _asplayer_controller
    (:Is%20Valid
      (Input|AddMappingContext (PlayerController|LocalPlayerSubsystems|GetEnhancedInputLocalPlayerSubsystem _asplayer_controller) "/Game/Blueprints/Input/IMC_DefaultCharacterInputContext.IMC_DefaultCharacterInputContext" 0 "(bIgnoreAllPressedKeysUntilRelease=True,bForceImmediately=False,bNotifyUserSettings=False)")
      (Input|AddMappingContext (PlayerController|LocalPlayerSubsystems|GetEnhancedInputLocalPlayerSubsystem _asplayer_controller) "/Game/Blueprints/AI/AITestBP/IMC_TestEquip.IMC_TestEquip" 0 "(bIgnoreAllPressedKeysUntilRelease=True,bForceImmediately=False,bNotifyUserSettings=False)"))))

(event EventTick
  (params (DeltaSeconds :type Float%20%28single-precision%29)))

(fn ConstructionScript)