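; BP_TestWeapon is a test weapon component for a player character that fires projectiles and supplies reload animations.
; InitWeapon caches the owning BTS_CharacterBase, finds its weapon skeletal mesh by component tag and prints debug info.
; Fire spawns BP_TestProjectile at the muzzle socket plus a camera-rotated offset, aimed along the camera rotation.
; GetReloadAnim returns the crouch or idle reload animation based on crouch state.
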(event EventBeginPlay)

(event EventTick
  (params (DeltaSeconds :type Float%20%28single-precision%29)))

(fn Fire
  (bind _returnvalue (Game|GetPlayerCameraManager 0))
  (bind _returnvalue_2 (Camera|GetCameraRotation _returnvalue))
  (Game|SpawnActorfromClass "/Game/Blueprints/Character/Player/BP_TestProjectile.BP_TestProjectile_C" (Math|Transform|MakeTransform (+ (Transformation|GetSocketLocation (Variables|Default|GetWeaponMesh) "MuzzleSocket") (Math|Vector|RotateVector (LocalVariables|GetOffset) _returnvalue_2)) _returnvalue_2) "Undefined" "OverrideRootScale" 0 0))

(fn GetReloadAnim
  (params (IsCrouch :type Boolean))
  (if IsCrouch
    (LocalVariables|SetReturnAnim (Variables|Default|GetReloadAnimCrouch))
    (else
      (LocalVariables|SetReturnAnim (Variables|Default|GetReloadAnimIdle))))
  (return (LocalVariables|GetReturnAnim)))

(fn InitWeapon
  (params (Owner :type Actor%20Object%20Reference))
  (bind _asbts_character_base (Utilities|Casting|CastToBTS_CharacterBase Owner))
  (bind _output_get (Variables|Default|SetOwner _asbts_character_base))
  (Variables|Default|SetWeaponMesh (Utilities|Array|Get(acopy) (Actor|GetComponentsbyTag _output_get "/Script/Engine.SkeletalMeshComponent" "TestWeapon")))
  (Development|PrintString (Utilities|GetDisplayName (Utilities|Array|Get(acopy) (Actor|GetComponentsbyTag _output_get "BP_TestWeapon_C" "TestWeaponComponent"))))
  (Development|PrintString (Utilities|String|ToString(Integer) (Utilities|Array|Length (Actor|GetComponentsbyTag _output_get "BP_TestWeapon_C" "TestWeaponComponent"))))
  (return))