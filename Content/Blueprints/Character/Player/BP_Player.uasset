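; Player character Blueprint handling grenade throws, interaction, parachuting, inventory, camera perspective and animation states.
; Holding T readies an attached grenade and redraws its predicted path with spline meshes each frame until release throws it.
; Tick traces from the first-person camera for interactables and overrides gravity, air control and fall speed while parachuting.
; BeginPlay creates the inventory widget and binds GAS attributes to the HUD through an overlay controller.
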(event Custom|ShowProjectilePath
  (|CollapseGraph_2))

(event Custom|InventoryTempInput
  (bind _returnvalue (Game|GetPlayerController 0))
  (bind _returnvalue_2 (Game|GetPlayerController 0))
  (bind _inventorywidget (Variables|Default|GetInventoryWidget))
  (if (UserInterface|Viewport|IsinViewport _inventorywidget)
    (Widget|RemovefromParent _inventorywidget)
    (Input|SetInputModeGameOnly _returnvalue_2 false)
    (Variables|/Script/Engine.PlayerController|SetbShowMouseCursor _returnvalue_2 false)
    (else
      (UserInterface|Viewport|AddtoViewport _inventorywidget 0)
      (Input|SetInputModeGameandUI _returnvalue (Variables|Default|GetInventoryWidget) "DoNotLock" false false)
      (Variables|/Script/Engine.PlayerController|SetbShowMouseCursor _returnvalue true))))

(event EventBeginPlay
  ;[1 1 1] 인벤토리 초기화
  (Input|EnableInput (Game|GetPlayerController 0))
  (Variables|Default|SetAnimationState "Unarmed")
  (bind _asbp_inventory_component (Utilities|Casting|CastToBP_InventoryComponent (Variables|Default|GetInventoryComponent)))
  (bind _returnvalue (UserInterface|CreateWidget "/Game/Blueprints/UI/InventoryWidget/WBP_InventoryWidget.WBP_InventoryWidget_C" (Game|GetPlayerController 0) _asbp_inventory_component 8e+01))
  (Variables|Default|SetInventoryWidget _returnvalue)
  (CallFunction|BindAttributetoWidget)
  (bind _asbp_parachute (Utilities|Casting|CastToBP_Parachute (Variables|/Script/Engine.ChildActorComponent|GetChildActor (Variables|Default|GetBag))))
  (Variables|Default|SetBP%20Parachute _asbp_parachute))

(event EventTick
  (params (DeltaSeconds :type Float%20%28single-precision%29))
  (Utilities|FlowControl|Sequence
    (:then_0
      (CallFunction|LineTraceTTP))
    (:then_1
      (CallFunction|SetGravity))))

(event EventSetAnimationState
  (params (NewState :type EAnimationState%20Enum :default "None"))
  (Variables|Default|SetAnimationState NewState))

(event EventChangePerspective
  (bind _charactermovement (Variables|Character|GetCharacterMovement))
  (Utilities|FlowControl|FlipFlop
    (:A
      (Components|Activation|SetActive (Variables|Components|GetFPP_Camera) true false)
      (Components|Activation|SetActive (Variables|Components|GetTTP_Camera) false false)
      (Variables|/Script/Engine.CharacterMovementComponent|SetbOrientRotationToMovement _charactermovement true))
    (:B
      (Components|Activation|SetActive (Variables|Components|GetFPP_Camera) false false)
      (Components|Activation|SetActive (Variables|Components|GetTTP_Camera) true false)
      (Variables|/Script/Engine.CharacterMovementComponent|SetbOrientRotationToMovement _charactermovement false))))

(event EventOnLanded
  (params (Hit :type Hit%20Result%20Structure%20%28by%20ref%29))
  (bind _charactermovement (Variables|Character|GetCharacterMovement))
  (bind _velocity (Variables|/Script/Engine.MovementComponent|GetVelocity _charactermovement))
  (bind _returnvalue (Math|Float|Absolute(Float) (.z _velocity)))
  (Utilities|FlowControl|Sequence
    (:then_0
      (if (Math|Float|InRange(Float) _returnvalue 3e+02 7.5e+02)
        (Variables|Default|SetOnLandState "NormalLand")))
    (:then_1
      (if (Math|Float|InRange(Float) _returnvalue 7.5e+02 1e+03)
        (Variables|Default|SetOnLandState "SoftLand")))
    (:then_2
      (if (> _returnvalue 1e+03)
        (Variables|Default|SetOnLandState "HardLand")))))

(event Input|KeyboardEvents|F
  (params (Key :type Key%20Structure :default "None"))
  (bind _interactable_actor (Variables|Default|GetInteractable%20Actor))
  (bind _interactable_actor_2 (Variables|Default|GetInteractable%20Actor))
  (:Pressed
    (Utilities|IsValid _interactable_actor
      (:Is%20Valid
        (Class|BTSInteractionInterface|Interaction(Message) _interactable_actor))))
  (:Released
    (Utilities|IsValid _interactable_actor_2
      (:Is%20Valid
        (Class|BTSInteractionInterface|InteractionClear(Message) _interactable_actor_2)))))

(event Input|KeyboardEvents|T
  (params (Key :type Key%20Structure :default "None"))
  (:Pressed
    (Animation|Montage|PlayMontage (Variables|Character|GetMesh) "/Game/Asset/Animation/Mixamo/AM_ThrowGranade1.AM_ThrowGranade1"
      (:then
        (bind _returnvalue (Game|SpawnActorfromClass "/Game/Blueprints/Item/BP_Granade.BP_Granade_C" (Math|Transform|MakeTransform (Transformation|GetSocketLocation (Variables|Character|GetMesh) "middle_01_r") "0, 0, 0" "1.000000,1.000000,1.000000") "AlwaysSpawn" "MultiplyWithRoot" 0 0))
        (bind _output_get (Variables|Default|SetBP%20Granade _returnvalue))
        (Transformation|AttachComponentToComponent _output_get (Variables|Character|GetMesh) "middle_01_r" "SnapToTarget" "SnapToTarget" "KeepWorld" true))
      (:OnNotifyBegin
        (Variables|Default|SetThrowing true)
        (CallFunction|ShowProjectilePath))))
  (:Released
    (if (Variables|Default|GetThrowing)
      (Animation|Montage|PlayMontage (Variables|Character|GetMesh) "/Game/Asset/Animation/Mixamo/AM_ThrowGranade1.AM_ThrowGranade1" 1.0 0.0 "End"
        (:then
          (Variables|Default|SetThrowing false)
          (Utilities|FlowControl|Delay 0.1)
          (Utilities|IsValid (Variables|Default|GetBP%20Granade)
            (:Is%20Valid
              (Default|Throw (Variables|Default|GetBP%20Granade) (Utilities|ThrowVelocity))))))
      (else
        (Animation|StopAnimMontage "/Game/Asset/Animation/Mixamo/AM_ThrowGranade1.AM_ThrowGranade1")
        (Utilities|IsValid (Variables|Default|GetBP%20Granade)
          (:Is%20Valid
            (Actor|DestroyActor (Variables|Default|GetBP%20Granade))))))))

(event Input|KeyboardEvents|7
  (params (Key :type Key%20Structure :default "None"))
  ;[1 1 1] Temp Anim State Change
  (:Pressed
    (Variables|Default|SetAnimationState "Unarmed")))

(event Input|KeyboardEvents|8
  (params (Key :type Key%20Structure :default "None"))
  ;[1 1 1] Temp Anim State Change
  (:Pressed
    (Variables|Default|SetAnimationState "Pistol")))

(event Input|KeyboardEvents|9
  (params (Key :type Key%20Structure :default "None"))
  ;[1 1 1] Temp Anim State Change
  (:Pressed
    (Variables|Default|SetAnimationState "Rifle")))

(fn ConstructionScript)

(fn GetPlayerController
  (bind _asplayer_controller (Utilities|Casting|CastToPlayerController (Pawn|GetController)))
  (return _asplayer_controller))

(fn LineTraceTTP
  (bind _fpp_camera (Variables|Components|GetFPP_Camera))
  (bind _returnvalue (Transformation|GetWorldLocation _fpp_camera))
  (bind (_outhit _returnvalue_2) (Collision|LineTraceByChannel _returnvalue (+ _returnvalue (* (Math|Vector|GetForwardVector (Transformation|GetWorldRotation _fpp_camera)) 2e+02)) "TraceTypeQuery4" true 0 "None" true "(R=1.000000,G=0.000000,B=0.000000,A=1.000000)" "(R=0.000000,G=1.000000,B=0.000000,A=1.000000)" 1.0))
  (if _returnvalue_2
    (if (Utilities|DoesObjectImplementInterface (.HitActor (Collision|BreakHitResult _outhit)) "/Script/BrutalTakedownSquad.BTS_InteractionInterface")
      (Class|BTSInteractionInterface|Visible(Message) (.HitActor (Collision|BreakHitResult _outhit)))
      (Variables|Default|SetInteractable%20Actor (.HitActor (Collision|BreakHitResult _outhit))))
    (else
      (Utilities|IsValid (Variables|Default|GetInteractable%20Actor)
        (:Is%20Valid
          (Class|BTSInteractionInterface|InteractionClear(Message) (Variables|Default|GetInteractable%20Actor))
          (Variables|Default|SetInteractable%20Actor 0))))))

(fn SetGravity
  (bind _returnvalue (Transformation|GetVelocity))
  (bind _charactermovement (Variables|Character|GetCharacterMovement))
  (bind _charactermovement_2 (Variables|Character|GetCharacterMovement))
  (bind _set_parachute (Variables|Default|GetSet%20Parachute))
  (bind (_x _y) (Math|Vector|BreakVector _returnvalue))
  (Default|SetParachuteVisible (Variables|Default|GetBP%20Parachute) _set_parachute)
  (if _set_parachute
    (Variables|/Script/Engine.CharacterMovementComponent|SetAirControl _charactermovement 2e+02)
    (Variables|/Script/Engine.CharacterMovementComponent|SetGravityScale _charactermovement 0.5)
    (Variables|/Script/Engine.MovementComponent|SetVelocity _charactermovement (Math|Vector|MakeVector _x _y -3e+02))
    (else
      (Variables|/Script/Engine.CharacterMovementComponent|SetAirControl _charactermovement_2 0.2)
      (Variables|/Script/Engine.CharacterMovementComponent|SetGravityScale _charactermovement_2 1.0))))

(fn GetWeaponComponent
  (return 0))

(fn BindAttributetoWidget
  (bind _asbp_player_hud_division (Utilities|Casting|CastToBP_PlayerHUD_Division (UserInterface|GetUserWidgetObject (Variables|Default|Get%20HUD%20Widget))))
  (Variables|Default|SetAs%20BP%20Player%20HUD%20Division _asbp_player_hud_division)
  (bind _returnvalue (Game|ConstructObjectfromClass self "/Game/Blueprints/UI/OverlayWidgetController/BP_OverlayWidgetController.BP_OverlayWidgetController_C"))
  (Variables|Default|SetOverlayWidger _returnvalue)
  (bind _returnvalue_2 (GameplayAttributes|GetAttributeSet (Ability|GetAbilitySystemComponent self) "/Script/BrutalTakedownSquad.BTS_AttributeSet"))
  (Class|BTSPlayerWidgetController|SetWidgetControllerParams (Variables|Default|GetOverlayWidger) (Utilities|Struct|MakeWidgetControllerParams (Game|GetPlayerController 0) (Game|GetPlayerState 0) _returnvalue_2 (Ability|GetAbilitySystemComponent self)))
  (Class|BTSOverlayWidgetController|BindCallbackstoDependenceies (Variables|Default|GetOverlayWidger))
  (Class|BTSPlayerUserWidget|SetWidgetController (Variables|Default|GetAs%20BP%20Player%20HUD%20Division) (Variables|Default|GetOverlayWidger))
  (Class|BTSOverlayWidgetController|BroadcastInitialValues (Variables|Default|GetOverlayWidger)))