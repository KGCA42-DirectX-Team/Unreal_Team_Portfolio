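; Player controller that sets up Enhanced Input for the player and relays the inventory toggle to the player pawn.
; On BeginPlay it adds the default character and inventory mapping contexts to the local player subsystem at equal priority.
; The inventory toggle action casts the first player's pawn to BP_Player and calls its temporary inventory input handler, printing an error if the cast fails.
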(event Input|EnhancedActionEvents|EnhancedInputActionIA_ToggleInventoryUI
  (params (ActionValue :type Boolean) (ElapsedSeconds :type Float%20%28double-precision%29) (TriggeredSeconds :type Float%20%28double-precision%29) (InputAction :type Input%20Action%20Object%20Reference :default "/Game/Blueprints/UI/TestPlayer/IA_ToggleInventoryUI.IA_ToggleInventoryUI"))
  (bind _asbp_player (Utilities|Casting|CastToBP_Player (Game|Player|GetPlayerPawn 0))
    (:then
      (Default|InventoryTempInput _asbp_player))
    (:CastFailed
      (Development|PrintString "PlayerController: cast failed to BP_Player"))))

(event EventBeginPlay
  (bind _self self)
  (bind _returnvalue (PlayerController|LocalPlayerSubsystems|GetEnhancedInputLocalPlayerSubsystem _self))
  (Utilities|IsValid _self
    (:Is%20Valid
      (Input|AddMappingContext _returnvalue "/Game/Blueprints/Input/IMC_DefaultCharacterInputContext.IMC_DefaultCharacterInputContext" 0 "(bIgnoreAllPressedKeysUntilRelease=True,bForceImmediately=False,bNotifyUserSettings=False)")
      (Input|AddMappingContext _returnvalue "/Game/Blueprints/UI/TestPlayer/IMC_Inventory.IMC_Inventory" 0 "(bIgnoreAllPressedKeysUntilRelease=True,bForceImmediately=False,bNotifyUserSettings=False)"))
    (:Is%20Not%20Valid
      (Development|PrintString "PlayerController: controller not vaild"))))

(fn ConstructionScript)