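; BP_ImageCapture is a utility Blueprint that frames a given static mesh for a portrait capture.
; GeneratePortrait assigns the mesh to its StaticMesh component, then sizes the 2D capture component's ortho width from the mesh's bounding sphere with a small margin.
; It offsets the capture along X from the bounds origin in proportion to the box extent and adds the mesh component to its show-only list.
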(event Custom|GeneratePortrait
  (params (Static%20Mesh :type Static%20Mesh%20Object%20Reference))
  (bind _returnvalue (StaticMesh|GetBounds Static%20Mesh))
  (Components|StaticMesh|SetStaticMesh (Variables|Default|GetStaticMesh) Static%20Mesh)
  (Variables|/Script/Engine.SceneCaptureComponent2D|SetOrthoWidth (Variables|DecalActor|GetCaptureComponent2D) (* (.sphereradius _returnvalue) 2.1))
  (Transformation|SetRelativeLocation (Variables|DecalActor|GetCaptureComponent2D) (+ (.origin _returnvalue) (Math|Vector|MakeVector (* (.x (.boxextent _returnvalue)) 3.0) 0.0 0.0)) false true)
  (Rendering|SceneCapture|ShowOnlyComponent (Variables|DecalActor|GetCaptureComponent2D) (Variables|Default|GetStaticMesh)))

(event EventBeginPlay)

(event EventTick
  (params (DeltaSeconds :type Float%20%28single-precision%29)))

(fn ConstructionScript)