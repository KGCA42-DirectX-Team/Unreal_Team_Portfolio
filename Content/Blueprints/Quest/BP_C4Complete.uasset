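; BP_C4Complete is a quest state for the completion stage of quest C4, which depends on the owner holding at least four of item 691.
; On Execute it reads that item's count from the quest owner's InventoryComponent.
; If the count is short, it switches the quest back to a newly constructed BP_C4Progress state; otherwise it sets the quest description to its QuestDescriptionString.
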(event EventExecute
  (if (< (.Value (Utilities|Map|Find (Variables|/Script/BrutalTakedownSquad.BTS_InventoryComponent|GetStoredItemCounts (Variables|/Script/BrutalTakedownSquad.BTS_CharacterBase|GetInventoryComponent (Class|BTSQuest|GetOwner (Variables|Default|GetQuest)))) "691")) 4)
    (bind _returnvalue (Game|ConstructObjectfromClass "/Game/Blueprints/Quest/BP_C4Progress.BP_C4Progress_C"))
    (Class|BTSQuest|SetState (Variables|Default|GetQuest) _returnvalue)
    (else
      (Class|BTSQuest|SetQuestDescription (Variables|Default|GetQuest) (Variables|Default|GetQuestDescriptionString)))))