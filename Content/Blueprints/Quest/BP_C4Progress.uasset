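; BP_C4Progress is a quest state that tracks collection of item 691 for the C4 quest.
; On Execute it reads the item's count from the quest owner's InventoryComponent and appends it to the base description while below four.
; Once the count reaches four, it constructs a BP_C4Complete state and hands it to the quest, while Enter and Exit only print debug strings.
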(event EventEnter
  (Development|PrintString 0 "C4 Progress Enger"))

(event EventExit
  (Development|PrintString 0 "C4 Progress Exit"))

(event EventExecute
  (bind _quest (Variables|Default|GetQuest))
  (bind _returnvalue (Class|BTSQuest|GetOwner _quest))
  (bind _inventorycomponent (Variables|/Script/BrutalTakedownSquad.BTS_CharacterBase|GetInventoryComponent _returnvalue))
  (bind _storeditemcounts (Variables|/Script/BrutalTakedownSquad.BTS_InventoryComponent|GetStoredItemCounts _inventorycomponent))
  (bind _value (Utilities|Map|Find _storeditemcounts "691"))
  (if (< _value 4)
    (Variables|Default|SetQuestDescriptionString (Utilities|String|Append (Variables|Default|GetBaseString) (Utilities|String|ToString(Integer) _value)))
    (else
      (bind _returnvalue_2 (Game|ConstructObjectfromClass "/Game/Blueprints/Quest/BP_C4Complete.BP_C4Complete_C"))
      (Class|BTSQuest|SetState (Variables|Default|GetQuest) _returnvalue_2))))