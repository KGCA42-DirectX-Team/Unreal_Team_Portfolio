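; BP_Ammo is an ammo pickup item that reacts to being made visible and to interaction.
; The Visible event briefly turns on custom depth rendering on the skeletal mesh, a short pulse that can serve as a highlight.
; Interaction calls ApplyEffect on the first player character, plays the rifle ammo pickup sound at the item's location and destroys the actor.
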(event EventVisible
  (Rendering|SetRenderCustomDepth (Variables|Default|GetSkeletalMesh) true)
  (Utilities|FlowControl|Delay 0.2)
  (Rendering|SetRenderCustomDepth (Variables|Default|GetSkeletalMesh) false))

(event EventInteraction
  (Class|BTSEffectActor|ApplyEffect (Game|GetPlayerCharacter 0))
  (Audio|SpawnSoundatLocation "/Game/Asset/MilitaryWeapSilver/Sound/Rifle/Cues/Rifle_AmmoPickup_Cue.Rifle_AmmoPickup_Cue" (Transformation|GetActorLocation) "0, 0, 0" 1.0 1.0 0.0 0 0)
  (Actor|DestroyActor))

(fn ConstructionScript)