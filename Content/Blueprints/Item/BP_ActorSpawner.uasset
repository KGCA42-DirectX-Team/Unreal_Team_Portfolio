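; BP_ActorSpawner is a placeable actor that spawns a weapon item into the world at its own transform.
; On BeginPlay it looks up its ItemID in the weapon data table and builds a BP_ItemObject from the row's dimensions and icons.
; It then spawns the row's item actor with that object, setting its skeletal mesh and name from the row.
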(event EventBeginPlay
  (bind _output_get (Variables|Default|SetWeaponDT "/Game/Blueprints/Item/WeaponDataTable.WeaponDataTable"))
  (bind _returnvalue (Utilities|GetDataTableRow _output_get (Variables|Default|GetItemID))
    (:then
      (bind _returnvalue_2 (Game|ConstructObjectfromClass "/Game/Blueprints/UI/Item/BP_ItemObject.BP_ItemObject_C" (.Dimensions (Utilities|Struct|BreakFWeapon _returnvalue)) (.Icon (Utilities|Struct|BreakFWeapon _returnvalue)) (.IconRotated (Utilities|Struct|BreakFWeapon _returnvalue))))
      (Variables|/Script/BrutalTakedownSquad.BTS_ItemObject|SetItemID _returnvalue_2 (Variables|Default|GetItemID))
      (bind _returnvalue_3 (Game|SpawnActorfromClass (.ItemActor (Utilities|Struct|BreakFWeapon _returnvalue)) (Transformation|GetActorTransform) "Undefined" "MultiplyWithRoot" 0 _returnvalue_2 0))
      (Components|SkeletalMesh|SetSkeletalMeshAsset (Variables|/Script/BrutalTakedownSquad.BTS_ItemUI|GetItemMesh _returnvalue_3) (.SKMeshAssetPath (Utilities|Struct|BreakFWeapon _returnvalue)))
      (Variables|/Script/BrutalTakedownSquad.BTS_ItemUI|SetItemName _returnvalue_3 (.Name (Utilities|Struct|BreakFWeapon _returnvalue))))))

(fn ConstructionScript)