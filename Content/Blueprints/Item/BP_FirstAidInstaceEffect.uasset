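; BP_FirstAidInstaceEffect is an interactable first aid item that applies an effect to the player and then destroys itself.
; Interaction passes player character 0 to ApplyEffect, whose logic is not defined in this graph.
; Visible highlights the skeletal mesh by enabling custom depth rendering for a fraction of a second.
; The box overlap checks for the Player tag but takes no action.
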(event OnComponentBeginOverlap(Box)
  (params (OverlappedComponent :type Primitive%20Component%20Object%20Reference) (OtherActor :type Actor%20Object%20Reference) (OtherComp :type Primitive%20Component%20Object%20Reference) (OtherBodyIndex :type Integer) (bFromSweep :type Boolean) (SweepResult :type Hit%20Result%20Structure%20%28by%20ref%29))
  (if (Actor|ActorHasTag OtherActor "Player")
    _))

(event EventInteraction
  (Class|BTSEffectActor|ApplyEffect (Game|GetPlayerCharacter 0))
  (Actor|DestroyActor))

(event EventVisible
  (Rendering|SetRenderCustomDepth (Variables|Default|GetSkeletalMesh) true)
  (Utilities|FlowControl|Delay 0.2)
  (Rendering|SetRenderCustomDepth (Variables|Default|GetSkeletalMesh) false))

(fn ConstructionScript)