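; BP_Item is a pickup actor that gives its ItemObject to any BTS_CharacterBase that overlaps its sphere.
; The overlap calls TryAddItem on the character's InventoryComponent, then destroys the actor on success or prints a failure message.
; Two unconnected chains remain unused: registering a weapon mesh from the item's data table row, and triggering an enemy's equip-weapon event after pickup.
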(event OnComponentBeginOverlap(Sphere)
  (params (OverlappedComponent :type Primitive%20Component%20Object%20Reference) (OtherActor :type Actor%20Object%20Reference) (OtherComp :type Primitive%20Component%20Object%20Reference) (OtherBodyIndex :type Integer) (bFromSweep :type Boolean) (SweepResult :type Hit%20Result%20Structure%20%28by%20ref%29))
  (bind _asbts_character_base (Utilities|Casting|CastToBTS_CharacterBase OtherActor))
  (Variables|Default|SetBTS%20Character%20Base _asbts_character_base)
  (if true
    (bind _returnvalue (Default|TryAddItem (Variables|/Game/Blueprints/Character/Player/BP_Player.BP_Player_C|GetInventoryComponent (Variables|Default|GetBTS%20Character%20Base)) (Variables|Default|GetItemObject)))
    (if _returnvalue
      (Actor|DestroyActor)
      (else
        (Development|PrintString "ItemUI: item not added")))))

(fn ConstructionScript)