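; BP_FirstAidKit is a world pickup that adds an item to the inventory of an overlapping BTS_CharacterBase.
; On BeginPlay it builds a 2x2 BP_ItemObject if none exists, though with AK47 icons and BP_AR15 as item class rather than first-aid content.
; Sphere overlap passes that object to the character's InventoryComponent, destroying the pickup on success and printing a message on failure.
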(event OnComponentBeginOverlap(Sphere)
  (params (OverlappedComponent :type Primitive%20Component%20Object%20Reference) (OtherActor :type Actor%20Object%20Reference) (OtherComp :type Primitive%20Component%20Object%20Reference) (OtherBodyIndex :type Integer) (bFromSweep :type Boolean) (SweepResult :type Hit%20Result%20Structure%20%28by%20ref%29))
  (bind _asbts_character_base (Utilities|Casting|CastToBTS_CharacterBase OtherActor))
  (bind _returnvalue (Default|TryAddItem (Variables|/Game/Blueprints/Character/Player/BP_Player.BP_Player_C|GetInventoryComponent _asbts_character_base) (Variables|Default|GetItemObject)))
  (if _returnvalue
    (Actor|DestroyActor)
    (else
      (Development|PrintString "ItemUI: item not added"))))

(event EventBeginPlay
  (if (not (Utilities|IsValid (Variables|Default|GetItemObject)))
    (CallFunction|ConstructItemObject)))

(fn ConstructionScript
  (|CallParentFunction))

(fn ConstructItemObject
  (bind _returnvalue (Game|ConstructObjectfromClass "/Game/Blueprints/UI/Item/BP_ItemObject.BP_ItemObject_C" (Utilities|Struct|MakeIntPoint 2 2) "/Game/Asset/FPS_Weapon_Bundle/Weapons/TempWeaponImage/MI_IconAk47.MI_IconAk47" "/Game/Asset/FPS_Weapon_Bundle/Weapons/TempWeaponImage/MI_IconAk47_R.MI_IconAk47_R" "/Game/Blueprints/Item/BP_AR15.BP_AR15_C"))
  (Variables|Default|SetItemObject _returnvalue)
  (return))