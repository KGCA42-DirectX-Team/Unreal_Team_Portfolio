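; Placeable spawner that creates a weapon or item actor at its own transform on BeginPlay, using the data table row named by ItemID.
; It builds a BP_ItemObject carrying the row's UI dimensions, icons and the ID, then passes it into the spawned actor.
; The actor class, skeletal mesh, name and type tag all come from that row, so one spawner serves any table entry.
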(event EventBeginPlay
  (bind _returnvalue (Utilities|GetDataTableRow (Variables|Default|GetDataTable) (Variables|Default|GetItemID))
    (:then
      (bind _returnvalue_2 (Game|ConstructObjectfromClass "/Game/Blueprints/UI/Item/BP_ItemObject.BP_ItemObject_C" (.UI_Dimensions (Utilities|Struct|BreakFWeapon _returnvalue)) (.UI_Icon (Utilities|Struct|BreakFWeapon _returnvalue)) (.UI_IconRotated (Utilities|Struct|BreakFWeapon _returnvalue))))
      (Variables|/Script/BrutalTakedownSquad.BTS_ItemObject|SetItemID _returnvalue_2 (Variables|Default|GetItemID))
      (bind _returnvalue_3 (Game|SpawnActorfromClass (.ItemBaseActorClass (Utilities|Struct|BreakFWeapon _returnvalue)) (Transformation|GetActorTransform) "Undefined" "MultiplyWithRoot" 0 _returnvalue_2 0))
      (Components|SkeletalMesh|SetSkeletalMeshAsset (Variables|/Script/BrutalTakedownSquad.BTS_ItemUI|GetItemMesh _returnvalue_3) (.SkeletalMeshAsset (Utilities|Struct|BreakFWeapon _returnvalue)))
      (Variables|/Script/BrutalTakedownSquad.BTS_ItemUI|SetItemName _returnvalue_3 (.Name (Utilities|Struct|BreakFWeapon _returnvalue)))
      (Variables|/Script/BrutalTakedownSquad.BTS_ItemUI|SetItemTypeTag _returnvalue_3 (.ItemType (Utilities|Struct|BreakFWeapon _returnvalue))))))

(fn ConstructionScript)