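; BP_AR15 is a deprecated rifle pickup that a character collects by overlapping its sphere.
; On BeginPlay it builds a grid-sized BP_ItemObject if none is set, using AK-47 icon materials.
; On overlap, it registers its mesh with the character's weapon component and fires the pickup event, then tries adding the item to the inventory.
; A failed add only prints a message, after the weapon is already registered.
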(event OnComponentBeginOverlap(Sphere)
  (params (OverlappedComponent :type Primitive%20Component%20Object%20Reference) (OtherActor :type Actor%20Object%20Reference) (OtherComp :type Primitive%20Component%20Object%20Reference) (OtherBodyIndex :type Integer) (bFromSweep :type Boolean) (SweepResult :type Hit%20Result%20Structure%20%28by%20ref%29))
  (bind _asbts_character_base (Utilities|Casting|CastToBTS_CharacterBase OtherActor))
  (Utilities|IsValid (Variables|/Script/BrutalTakedownSquad.BTS_CharacterBase|GetWeaponComponent _asbts_character_base)
    (:Is%20Valid
      (bind _asbp_weapon_component (Utilities|Casting|CastToBP_WeaponComponent (Variables|/Script/BrutalTakedownSquad.BTS_CharacterBase|GetWeaponComponent _asbts_character_base)))
      (Default|RegisterWeapon _asbp_weapon_component (Variables|Default|GetItemMesh))
      (Default|OnPickUpEvent _asbp_weapon_component)
      (bind _returnvalue (Default|TryAddItem (Variables|/Game/Blueprints/Character/Player/BP_Player.BP_Player_C|GetInventoryComponent _asbts_character_base) (Variables|Default|GetItemObject)))
      (if (not _returnvalue)
        (Development|PrintString "ItemUI: item not added")))))

(event EventBeginPlay
  (if (not (Utilities|IsValid (Variables|Default|GetItemObject)))
    (CallFunction|ConstructItemObject)))

(fn ConstructionScript)

(fn ConstructItemObject
  (bind _returnvalue (Game|ConstructObjectfromClass "/Game/Blueprints/UI/Item/BP_ItemObject.BP_ItemObject_C" (Utilities|Struct|MakeIntPoint 8 3) "/Game/Asset/FPS_Weapon_Bundle/Weapons/TempWeaponImage/MI_IconAk47.MI_IconAk47" "/Game/Asset/FPS_Weapon_Bundle/Weapons/TempWeaponImage/MI_IconAk47_R.MI_IconAk47_R" 0))
  (Variables|Default|SetItemObject _returnvalue)
  (return))