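; BP_C4Case is a C4 case item that the player can pick up into a grid inventory.
; On BeginPlay it constructs a 4x6 BP_ItemObject if none is set, using the AK-47 icon materials.
; Visible briefly enables custom depth on the mesh, likely for a highlight.
; Interaction passes the item to player 0's InventoryComponent and destroys the actor on success, otherwise printing a failure message.
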(event EventBeginPlay
  (Utilities|IsValid (Variables|Default|GetItemObject)
    (:Is%20Not%20Valid
      (bind _returnvalue (Game|ConstructObjectfromClass "/Game/Blueprints/UI/Item/BP_ItemObject.BP_ItemObject_C" (Utilities|Struct|MakeIntPoint 4 6) "/Game/Asset/FPS_Weapon_Bundle/Weapons/TempWeaponImage/MI_IconAk47.MI_IconAk47" "/Game/Asset/FPS_Weapon_Bundle/Weapons/TempWeaponImage/MI_IconAk47_R.MI_IconAk47_R"))
      (Variables|Default|SetItemObject _returnvalue))))

(event EventVisible
  (Rendering|SetRenderCustomDepth (Variables|Default|GetItemMesh) true)
  (Utilities|FlowControl|Delay 0.2)
  (Rendering|SetRenderCustomDepth (Variables|Default|GetItemMesh) false))

(event EventInteraction
  (bind _asbts_character_base (Utilities|Casting|CastToBTS_CharacterBase (Game|GetPlayerCharacter 0)))
  (bind _returnvalue (Default|TryAddItem (Variables|/Game/Blueprints/Character/Player/BP_Player.BP_Player_C|GetInventoryComponent _asbts_character_base) (Variables|Default|GetItemObject)))
  (if _returnvalue
    (Actor|DestroyActor)
    (else
      (Development|PrintString "ItemUI: item not added"))))

(fn ConstructionScript
  (|CallParentFunction))