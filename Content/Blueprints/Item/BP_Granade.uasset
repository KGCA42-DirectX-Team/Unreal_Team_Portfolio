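; BP_Granade is a thrown grenade that explodes on a timer and applies radial damage through GAS.
; Throw detaches it, launches it with ProjectileMovement while randomly rotating the mesh, then briefly later enables sphere collision and hands velocity to physics simulation.
; After the fuse delay it spawns an explosion, sphere-traces for BTS_CharacterBase hits, applies GE_ExplosionDamage with a distance-scaled SetByCaller magnitude, and destroys itself.
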(event Custom|Throw
  (params (Velocity :type Vector))
  (bind _returnvalue (Transformation|GetActorLocation))
  (bind _projectilemovement (Variables|Default|GetProjectileMovement))
  (bind _sphere (Variables|Default|GetSphere))
  (Utilities|FlowControl|DoOnce false
    (:Completed
      (Utilities|FlowControl|Sequence
        (:then_0
          (Transformation|DetachFromActor "KeepWorld" "KeepWorld" "KeepWorld")
          (Variables|/Script/Engine.MovementComponent|SetVelocity _projectilemovement Velocity)
          (Components|Activation|Activate _projectilemovement false)
          (Utilities|FlowControl|Delay 0.2)
          (Collision|SetCollisionEnabled (Variables|Default|GetSphere) "QueryAndPhysics")
          (bind _output_get (Variables|Default|Setvelocity (Transformation|GetVelocity)))
          (Physics|SetSimulatePhysics _sphere true)
          (Physics|SetPhysicsLinearVelocity _sphere _output_get false "None")
          (Utilities|FlowControl|Delay 2.0)
          (Effects|SpawnEmitteratLocation "/Game/Asset/Realistic_Starter_VFX_Pack_Vol2/Particles/Explosion/P_Explosion_Big_A.P_Explosion_Big_A" _returnvalue)
          (CallFunction|SphereTrace _returnvalue _returnvalue))
        (:then_1
          (Components|MoveComponentTo (Variables|Default|GetSkeletalMesh) "0, 0, 0" (Math|Random|RandomRotator false) false false 0.5 false))))))

(event EventBeginPlay)

(event Collision|EventActorBeginOverlap
  (params (OtherActor :type Actor%20Object%20Reference)))

(event EventTick
  (params (DeltaSeconds :type Float%20%28single-precision%29)))

(fn ConstructionScript
  (Collision|SetCollisionEnabled (Variables|Default|GetSphere) "NoCollision"))

(fn SphereTrace
  (params (End :type Vector) (Start :type Vector))
  (bind _outhits (Collision|MultiSphereTraceByChannel Start End 8e+02 "TraceTypeQuery2" false 0 "ForDuration"))
  (for _array_element _outhits
    (bind _asbts_character_base (Utilities|Casting|CastToBTS_CharacterBase (.HitActor (Collision|BreakHitResult _array_element))))
    (bind _returnvalue (Ability|GameplayEffect|AssignTagSetbyCallerMagnitude (GameplayEffects|MakeOutgoingSpec :self (Ability|GetAbilitySystemComponent _asbts_character_base) :GameplayEffectClass "/Game/Blueprints/AbilitySystem/Effect/GE_ExplosionDamage.GE_ExplosionDamage_C") "(TagName=\"ExplosionDamage\")" (+ (* (/ (Math|Vector|Distance(Vector) (Transformation|GetActorLocation _asbts_character_base) (Transformation|GetActorLocation)) 1e+02) -1.0) 8.0)))
    (GameplayEffects|ApplyGameplayEffectSpecToSelf (Ability|GetAbilitySystemComponent _asbts_character_base) _returnvalue))
  (Actor|DestroyActor))