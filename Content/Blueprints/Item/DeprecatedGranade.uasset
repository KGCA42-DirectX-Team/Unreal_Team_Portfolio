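; Deprecated grenade item that throws itself along its forward vector at BeginPlay and shows an explosion after a short fuse.
; A once-only Throw event activates ProjectileMovement with the given velocity, then after a delay runs a debug-drawn multi sphere trace and spawns the explosion emitter.
; In parallel, it turns ItemMesh to a random rotation.
; The trace results are unused, so no damage is applied.
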(event Custom|Throw
  (params (Velocity :type Vector))
  (bind _projectilemovement (Variables|Default|GetProjectileMovement))
  (Utilities|FlowControl|DoOnce false
    (:Completed
      (Utilities|FlowControl|Sequence
        (:then_0
          (Variables|/Script/Engine.MovementComponent|SetVelocity _projectilemovement Velocity)
          (Components|Activation|Activate _projectilemovement false)
          (Utilities|FlowControl|Delay 2.0)
          (Collision|MultiSphereTraceByChannel "0, 0, 0" "0, 0, 0" 5e+02 "TraceTypeQuery2" false 0 "ForDuration")
          (Effects|SpawnEmitteratLocation "/Game/Asset/Realistic_Starter_VFX_Pack_Vol2/Particles/Explosion/P_Explosion_Big_A.P_Explosion_Big_A" (Transformation|GetActorLocation)))
        (:then_1
          (Components|MoveComponentTo (Variables|Default|GetItemMesh) "0, 0, 0" (Math|Random|RandomRotator false) false false 0.5 false))))))

(event EventBeginPlay
  (CallFunction|Throw (* (Transformation|GetActorForwardVector) 1.5e+03)))

(event Collision|EventActorBeginOverlap
  (params (OtherActor :type Actor%20Object%20Reference)))

(event EventTick
  (params (DeltaSeconds :type Float%20%28single-precision%29)))

(fn ConstructionScript
  (|CallParentFunction))