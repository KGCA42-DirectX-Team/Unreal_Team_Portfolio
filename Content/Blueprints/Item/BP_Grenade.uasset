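; BP_Grenade is a thrown grenade that warns nearby enemies to evade, then explodes and damages characters.
; Throw detaches it, launches it with ProjectileMovement, then hands velocity to sphere physics after a short delay; bounce sounds are capped.
; A timed sphere trace calls CallEvadeGranade on enemies before detonation effects play.
; SphereTrace line-traces toward character bones, applying GAS set-by-caller damage plus radial damage for each character hit.
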(event OnComponentHit(Sphere)
  (params (HitComponent :type Primitive%20Component%20Object%20Reference) (OtherActor :type Actor%20Object%20Reference) (OtherComp :type Primitive%20Component%20Object%20Reference) (NormalImpulse :type Vector :default "0, 0, 0") (Hit :type Hit%20Result%20Structure%20%28by%20ref%29))
  (Utilities|FlowControl|DoN 4
    (:Exit
      (Audio|PlaySoundatLocation "/Game/Asset/MilitaryWeapSilver/Sound/GrenadeLauncher/Cues/GrenadeLauncher_Bounce_Cue.GrenadeLauncher_Bounce_Cue" (Transformation|GetActorLocation) "0, 0, 0" 1.0 1.0 0.0 0 0 0 0))))

(event Custom|Throw
  (params (Velocity :type Vector))
  (bind _returnvalue (Transformation|GetActorLocation))
  (bind _returnvalue_2 (Transformation|GetActorLocation))
  (bind _projectilemovement (Variables|Default|GetProjectileMovement))
  (bind _sphere (Variables|Default|GetSphere))
  (Utilities|FlowControl|DoOnce false
    (:Completed
      (Utilities|FlowControl|Sequence
        (:then_0
          (Transformation|DetachFromActor "KeepWorld" "KeepWorld" "KeepWorld")
          (Variables|/Script/Engine.MovementComponent|SetVelocity _projectilemovement Velocity)
          (Components|Activation|Activate _projectilemovement false)
          (Utilities|FlowControl|Delay 0.2)
          (Collision|SetCollisionEnabled (Variables|Default|GetSphere) "QueryAndPhysics")
          (bind _output_get (Variables|Default|Setvelocity (Transformation|GetVelocity)))
          (Physics|SetSimulatePhysics _sphere true)
          (Physics|SetPhysicsLinearVelocity _sphere _output_get false "None")
          (Utilities|FlowControl|Delay 1.0)
          (bind _outhits (Collision|MultiSphereTraceByChannel _returnvalue _returnvalue 8e+02 "TraceTypeQuery1" false 0 "ForDuration" true "(R=0.000000,G=0.888169,B=1.000000,A=1.000000)" "(R=0.000000,G=0.037499,B=1.000000,A=1.000000)"))
          (bind _output_get_2 (Variables|Default|SetOut%20Hits _outhits))
          (for _array_element _output_get_2
            (bind _asbp_enemy_base (Utilities|Casting|CastToBP_EnemyBase (.HitActor (Collision|BreakHitResult _array_element))))
            (Default|CallEvadeGranade _asbp_enemy_base self))
          (Utilities|FlowControl|Delay 1.0)
          (Effects|SpawnEmitteratLocation "/Game/Asset/Realistic_Starter_VFX_Pack_Vol2/Particles/Explosion/P_Explosion_Big_A.P_Explosion_Big_A" _returnvalue_2)
          (Audio|PlaySoundatLocation "/Game/Asset/MilitaryWeapSilver/Sound/GrenadeLauncher/Cues/GrenadeLauncher_Explosion_Cue.GrenadeLauncher_Explosion_Cue" _returnvalue_2 "0, 0, 0" 1.0 1.0 0.0 0 0 0 0)
          (CallFunction|SphereTrace _returnvalue_2 _returnvalue_2)
          (Actor|DestroyActor))
        (:then_1
          (Components|MoveComponentTo (Variables|Default|GetSkeletalMesh) "0, 0, 0" (Math|Random|RandomRotator false) false false 0.5 false))))))

(event EventBeginPlay)

(event Collision|EventActorBeginOverlap
  (params (OtherActor :type Actor%20Object%20Reference)))

(event EventTick
  (params (DeltaSeconds :type Float%20%28single-precision%29)))

(fn ConstructionScript
  (Collision|SetCollisionEnabled (Variables|Default|GetSphere) "NoCollision"))

(fn SphereTrace
  (params (End :type Vector) (Start :type Vector))
  (bind _returnvalue (Transformation|GetActorLocation))
  (for _array_element (Variables|Default|GetOut%20Hits)
    (bind _asbts_character_base (Utilities|Casting|CastToBTS_CharacterBase (.HitActor (Collision|BreakHitResult _array_element))))
    (for _array_element_2 (Variables|Default|GetBoneName)
      (bind _outhit (Collision|LineTraceByChannel _returnvalue (+ _returnvalue (* (Math|Vector|GetUnitDirection(Vector) _returnvalue (Transformation|GetSocketLocation (Variables|/Script/Engine.Character|GetMesh _asbts_character_base) _array_element_2)) 6e+02)) "TraceTypeQuery2" false (Utilities|Array|MakeArray (Components|GetOwner self)) "ForDuration"))
      (bind _asbts_character_base_2 (Utilities|Casting|CastToBTS_CharacterBase (.HitActor (Collision|BreakHitResult _outhit))))
      (bind _returnvalue_2 (Ability|GameplayEffect|AssignTagSetbyCallerMagnitude (GameplayEffects|MakeOutgoingSpec :self (Ability|GetAbilitySystemComponent _asbts_character_base_2) :GameplayEffectClass "/Game/Blueprints/AbilitySystem/Effect/GE_ExplosionDamage.GE_ExplosionDamage_C") "(TagName=\"Attributes.Meta.ExplosionDamage\")" 2e+01))
      (GameplayEffects|ApplyGameplayEffectSpecToSelf (Ability|GetAbilitySystemComponent _asbts_character_base_2) _returnvalue_2)
      (Game|Damage|ApplyRadialDamage 1.0 (Transformation|GetActorLocation) 8e+02 0 0 self 0 false "ECC_Visibility"))))