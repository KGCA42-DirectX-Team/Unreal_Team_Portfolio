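; First aid kit pickup actor that heals any BTS_CharacterBase overlapping its sphere.
; Overlap plays a medkit montage on the character; on completion it applies a GAS heal effect via SetByCaller magnitude, spawns a grenade explosion emitter and destroys itself.
; The construction script builds an inventory item object, with a BeginPlay fallback that uses AK47 icons.
; The add-to-inventory logic is disconnected and never runs.
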(event OnComponentBeginOverlap(Sphere)
  (params (OverlappedComponent :type Primitive%20Component%20Object%20Reference) (OtherActor :type Actor%20Object%20Reference) (OtherComp :type Primitive%20Component%20Object%20Reference) (OtherBodyIndex :type Integer) (bFromSweep :type Boolean) (SweepResult :type Hit%20Result%20Structure%20%28by%20ref%29))
  (bind _asbts_character_base (Utilities|Casting|CastToBTS_CharacterBase OtherActor))
  (Animation|Montage|PlayMontage (Variables|/Script/Engine.Character|GetMesh _asbts_character_base) "/Game/Asset/Animation/Mixamo/AM_Medikit.AM_Medikit"
    (:OnCompleted
      (bind _returnvalue (Ability|GameplayEffect|AssignTagSetbyCallerMagnitude (GameplayEffects|MakeOutgoingSpec :self (Ability|GetAbilitySystemComponent _asbts_character_base) :GameplayEffectClass "/Game/Blueprints/AI/AITestBP/GE_TestHeal.GE_TestHeal_C") "(TagName=\"Tests.Healing\")" (Variables|Default|GetHeal)))
      (GameplayEffects|ApplyGameplayEffectSpecToSelf (Ability|GetAbilitySystemComponent _asbts_character_base) _returnvalue)
      (Effects|SpawnEmitteratLocation "/Game/Asset/MilitaryWeapSilver/FX/P_Grenade_Explosion_01.P_Grenade_Explosion_01" (Transformation|GetActorLocation))
      (Actor|DestroyActor))))

(event EventBeginPlay
  (if (not (Utilities|IsValid (Variables|Default|GetItemObject)))
    (CallFunction|ConstructItemObject)))

(fn ConstructionScript
  (bind _returnvalue (Game|ConstructObjectfromClass "/Game/Blueprints/UI/Item/BP_ItemObject.BP_ItemObject_C" (Utilities|Struct|MakeIntPoint 2 2) "/Game/Asset/FirstAidKit/MT_FirstAidKit.MT_FirstAidKit" "/Game/Asset/FirstAidKit/MT_FirstAidKitRotate.MT_FirstAidKitRotate"))
  (Variables|Default|SetItemObject _returnvalue))

(fn ConstructItemObject
  (bind _returnvalue (Game|ConstructObjectfromClass "/Game/Blueprints/UI/Item/BP_ItemObject.BP_ItemObject_C" (Utilities|Struct|MakeIntPoint 2 2) "/Game/Asset/FPS_Weapon_Bundle/Weapons/TempWeaponImage/MI_IconAk47.MI_IconAk47" "/Game/Asset/FPS_Weapon_Bundle/Weapons/TempWeaponImage/MI_IconAk47_R.MI_IconAk47_R"))
  (Variables|Default|SetItemObject _returnvalue)
  (return))