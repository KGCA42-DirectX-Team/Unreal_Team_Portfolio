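; BP_Projectile is a projectile that deals hit-location-based damage to characters through the Gameplay Ability System, with its mesh shown shortly after spawn.
; On a character hit, the physical material scales damage for head, body, arm or leg, then feeds a SetByCaller effect and reports an AI damage event.
; Non-character hits destroy the projectile; character hits do not destroy it here.
; An older effect-and-impulse chain remains unconnected.
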(event EventBeginPlay
  (Utilities|FlowControl|Delay 0.1)
  (Rendering|SetVisibility (Variables|Default|GetStaticMesh) true false))

(event Collision|EventHit
  (params (MyComp :type Primitive%20Component%20Object%20Reference) (Other :type Actor%20Object%20Reference) (OtherComp :type Primitive%20Component%20Object%20Reference) (bSelfMoved :type Boolean) (HitLocation :type Vector :default "0, 0, 0") (HitNormal :type Vector :default "0, 0, 0") (NormalImpulse :type Vector :default "0, 0, 0") (Hit :type Hit%20Result%20Structure%20%28by%20ref%29))
  (bind _physmat (Collision|BreakHitResult Hit))
  (bind _asbts_character_base (Utilities|Casting|CastToBTS_CharacterBase Other)
    (:then
      (Utilities|FlowControl|Sequence
        (:then_0
          (if (== _physmat "/Game/Data/PhysicalMaterial/Body/PM_Head.PM_Head")
            (Variables|Default|SetFinalDamage (* (Variables|Default|GetFinalDamage) 2.0))
            (Class|BTSEffectActor|SetCallerMagnitude "(TagName=\"Attributes.Meta.Damage\")" (Variables|Default|GetFinalDamage) "ALL" :!label _label)
            (Class|BTSEffectActor|ApplyEffect _asbts_character_base)
            (Class|AISenseDamage|ReportDamageEvent _asbts_character_base self 1.0 (Transformation|GetActorLocation) "0, 0, 0" "None")
            (elif (== _physmat "/Game/Data/PhysicalMaterial/Body/PM_Body.PM_Body")
              (goto _label)
              (elif (== _physmat "/Game/Data/PhysicalMaterial/Body/PM_Arm.PM_Arm")
                (Variables|Default|SetFinalDamage (* (Variables|Default|GetFinalDamage) 0.5))
                (goto _label)
                (elif (== _physmat "/Game/Data/PhysicalMaterial/Body/PM_Leg.PM_Leg")
                  (Variables|Default|SetFinalDamage (* (Variables|Default|GetFinalDamage) 0.25))
                  (goto _label))))))))
    (:CastFailed
      (Actor|DestroyActor))))

(fn ConstructionScript)