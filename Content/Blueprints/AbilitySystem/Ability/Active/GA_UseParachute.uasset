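; Gameplay ability that deploys the player's parachute while falling.
; On activation, if player 0 is falling without a parachute set, it sets the parachute flag, shows the Bag, binds a landing callback and ends the ability.
; The landing callback clears the flag, hides the Bag and plays a forward dive-roll montage.
; DoOnce nodes guard both deployment and the landing visuals.
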(event Custom|EndParachute
  (params (Hit :type Hit%20Result%20Structure%20%28by%20ref%29))
  (bind _as_bp_player (Variables|Default|GetAs%20BP%20Player))
  (Variables|/Game/Blueprints/Character/Player/BP_Player.BP_Player_C|SetSet%20Parachute _as_bp_player false)
  (Utilities|FlowControl|DoOnce false
    (:Completed
      (Rendering|SetVisibility (Variables|/Game/Blueprints/Character/Player/BP_Player.BP_Player_C|GetBag _as_bp_player) false false)
      (Animation|PlayAnimMontage (Variables|Default|GetAs%20BP%20Player) "/Game/Asset/Animation/Parachute/AM_DiveRollF.AM_DiveRollF" 1.0 "None"))))

(event Ability|EventActivateAbility
  (bind _asbp_player (Utilities|Casting|CastToBP_Player (Game|GetPlayerCharacter 0)))
  (Variables|Default|SetAs%20BP%20Player _asbp_player)
  (if (not (Variables|/Game/Blueprints/Character/Player/BP_Player.BP_Player_C|GetSet%20Parachute _asbp_player))
    (if (AI|Components|NavMovement|IsFalling (Variables|/Script/Engine.Character|GetCharacterMovement _asbp_player))
      (Utilities|FlowControl|DoOnce false
        (:Completed
          (Variables|/Game/Blueprints/Character/Player/BP_Player.BP_Player_C|SetSet%20Parachute (Variables|Default|GetAs%20BP%20Player) true)
          (Rendering|SetVisibility (Variables|/Game/Blueprints/Character/Player/BP_Player.BP_Player_C|GetBag (Variables|Default|GetAs%20BP%20Player)) true false)
          (EventDispatchers|BindEventtoLandedDelegate (Variables|Default|GetAs%20BP%20Player) (delegate Custom|EndParachute))
          (Ability|EndAbility))))))

(event Ability|EventOnEndAbility
  (params (bWasCancelled :type Boolean)))