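; Active gameplay ability for a melee attack that damages the first pawn struck in front of the character.
; OnMeleeAttackStart runs a capsule trace from the right hand socket along the actor's forward vector, with debug drawing on.
; On a hit, it applies GE_Damage to the target's ability system with a fixed set-by-caller magnitude, then waits briefly before ending.
; A miss ends the ability immediately.
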(event Ability|EventActivateAbility)

(event Ability|EventOnEndAbility
  (params (bWasCancelled :type Boolean)))

(event EventOnMeleeAttackStart
  (bind _returnvalue (Class|BTSCharacterMeleeAttack|GetCharacter))
  (bind _returnvalue_2 (Class|BTSCharacterMeleeAttack|GetCharacter))
  (bind _returnvalue_3 (Ability|GetAbilitySystemComponent _returnvalue))
  (bind _mesh (Variables|/Script/Engine.Character|GetMesh _returnvalue_2))
  (bind _returnvalue_4 (Transformation|GetSocketLocation _mesh "hand_r"))
  (bind _outhit (Class|KismetSystemLibrary|CapsuleTraceSingleforObjects _returnvalue_4 (+ _returnvalue_4 (* (Transformation|GetActorForwardVector _returnvalue_2) 1.5e+02)) 48.0 96.0 (Utilities|Array|MakeArray "ObjectTypeQuery3") false (Utilities|Array|MakeArray (Class|BTSCharacterMeleeAttack|GetCharacter)) "ForDuration" true))
  (if (Utilities|IsValid (.hitactor _outhit))
    (bind _returnvalue_5 (Ability|GameplayEffect|AssignTagSetbyCallerMagnitude (GameplayEffects|MakeOutgoingSpec _returnvalue_3 "/Game/Blueprints/AbilitySystem/Effect/GE_Damage.GE_Damage_C" 1.0 (GameplayEffects|MakeEffectContext _returnvalue_3)) "(TagName=\"Damage\")" 5e+01))
    (GameplayEffects|ApplyGameplayEffectSpecToSelf (Ability|GetAbilitySystemComponent (.hitactor _outhit)) _returnvalue_5)
    (Utilities|FlowControl|Delay 1.0))
  (Ability|EndAbility))