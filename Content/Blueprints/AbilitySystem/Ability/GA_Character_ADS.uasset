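; GA_Character_ADS is a gameplay ability that handles the player's aim-down-sights camera transition.
; Activation sets the player's ADS state and starts a tick task that advances a timer, setting spring arm length from the RifleADS curve table row until TimeLag elapses.
; ReleaseADS runs the timer backward along the same curve, then ends the ability.
; An interrupted transition stops the running tick task and reverses from its current time.
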(event Ability|EventActivateAbility
  (if (Variables|Default|GetIsFinishTask)
    (Variables|Default|SetADSTime 0.0)
    (else
      (Utilities|IsValid (Variables|Default|GetTIckTask)
        (:Is%20Valid
          (GameplayTasks|EndTask (Variables|Default|GetTIckTask)))
        (:Is%20Not%20Valid
          _))))
  (Class|AnimationEnumInterface|SetIsADS (Variables|Default|GetPlayer) true)
  (Variables|Default|SetIsFinishTask false)
  (bind (_asynctaskproxy _deltatime) (|AbilityTaskonTick "OnADS")
    (:then
      (Variables|Default|SetTIckTask _asynctaskproxy))
    (:OnTick
      (Variables|Default|SetADSTime (+ _deltatime (Variables|Default|GetADSTime)))
      (bind _outxy (DataTable|EvaluateCurveTableRow "/Game/Data/AnimData/ADSTimeCurve.ADSTimeCurve" "RifleADS" (Variables|Default|GetADSTime))
        (:RowFound
          (Variables|/Script/Engine.SpringArmComponent|SetTargetArmLength (Variables|/Script/BrutalTakedownSquad.BTS_Player|GetSpringArmComponent (Variables|Default|GetPlayer)) _outxy))
        (:RowNotFound
          _))
      (if (> (Variables|Default|GetADSTime) (Variables|Default|GetTimeLag))
        (Utilities|IsValid (Variables|Default|GetTIckTask)
          (:Is%20Valid
            (GameplayTasks|EndTask (Variables|Default|GetTIckTask))
            (Variables|Default|SetIsFinishTask true))
          (:Is%20Not%20Valid
            (Variables|Default|SetIsFinishTask true)))))))

(event EventReleaseADS
  (if (Variables|Default|GetIsFinishTask)
    (Variables|Default|SetADSTime (Variables|Default|GetTimeLag))
    (else
      (Utilities|IsValid (Variables|Default|GetTIckTask)
        (:Is%20Valid
          (GameplayTasks|EndTask (Variables|Default|GetTIckTask)))
        (:Is%20Not%20Valid
          _))))
  (Class|AnimationEnumInterface|SetIsADS (Variables|Default|GetPlayer) false)
  (Variables|Default|SetIsFinishTask false)
  (bind (_asynctaskproxy _deltatime) (|AbilityTaskonTick "EndADS")
    (:then
      (Variables|Default|SetTIckTask _asynctaskproxy))
    (:OnTick
      (Variables|Default|SetADSTime (- (Variables|Default|GetADSTime) _deltatime))
      (bind _outxy (DataTable|EvaluateCurveTableRow "/Game/Data/AnimData/ADSTimeCurve.ADSTimeCurve" "RifleADS" (Variables|Default|GetADSTime))
        (:RowFound
          (Variables|/Script/Engine.SpringArmComponent|SetTargetArmLength (Variables|/Script/BrutalTakedownSquad.BTS_Player|GetSpringArmComponent (Variables|Default|GetPlayer)) _outxy))
        (:RowNotFound
          _))
      (if (< (Variables|Default|GetADSTime) 0.0)
        (Utilities|IsValid (Variables|Default|GetTIckTask)
          (:Is%20Valid
            (GameplayTasks|EndTask (Variables|Default|GetTIckTask))
            (Variables|Default|SetIsFinishTask true)
            (Ability|EndAbility))
          (:Is%20Not%20Valid
            (Variables|Default|SetIsFinishTask true)
            (Ability|EndAbility)))))))