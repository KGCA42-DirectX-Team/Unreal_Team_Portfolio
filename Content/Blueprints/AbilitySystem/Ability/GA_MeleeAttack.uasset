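; GA_MeleeAttack is a Gameplay Ability that deals damage with a single forward melee hit.
; OnMeleeAttackStart runs a capsule trace for Pawns from the character's hand_r socket along its forward vector, with timed debug drawing.
; A hit actor's Ability System Component applies GE_Damage to itself, then the ability waits briefly before ending; a miss ends it immediately.
; ActivateAbility and OnEndAbility are empty.
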(event Ability|EventActivateAbility)

(event Ability|EventOnEndAbility
  (params (bWasCancelled :type Boolean)))

(event EventOnMeleeAttackStart
  (bind _returnvalue (Class|BTSCharacterMeleeAttack|GetCharacter))
  (bind _mesh (Variables|/Script/Engine.Character|GetMesh _returnvalue))
  (bind _returnvalue_2 (Transformation|GetSocketLocation _mesh "hand_r"))
  (bind _outhit (Class|KismetSystemLibrary|CapsuleTraceSingleforObjects _returnvalue_2 (+ _returnvalue_2 (* (Transformation|GetActorForwardVector _returnvalue) 1.5e+02)) 48.0 96.0 (Utilities|Array|MakeArray "ObjectTypeQuery3") false (Utilities|Array|MakeArray (Class|BTSCharacterMeleeAttack|GetCharacter)) "ForDuration" true))
  (if (Utilities|IsValid (.hitactor _outhit))
    (GameplayEffects|ApplyGameplayEffectToSelf :self (Ability|GetAbilitySystemComponent (.hitactor _outhit)) :GameplayEffectClass "/Game/Blueprints/AbilitySystem/Effect/GE_Damage.GE_Damage_C")
    (Utilities|FlowControl|Delay 1.0))
  (Ability|EndAbility))