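; BP_C4Real is an interactable C4 map object that adds trigger-line detection and interaction audio to its parent's behavior.
; Actors tagged Player that overlap TriggerLine are passed to TriggerLineOverlap, whose logic is not defined in this graph.
; Interaction calls the parent, then spawns a 2D data-loading sound and stores its AudioComponent.
; That sound is stopped when the interaction clears or the actor is destroyed.
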(event OnComponentBeginOverlap(TriggerLine)
  (params (OverlappedComponent :type Primitive%20Component%20Object%20Reference) (OtherActor :type Actor%20Object%20Reference) (OtherComp :type Primitive%20Component%20Object%20Reference) (OtherBodyIndex :type Integer) (bFromSweep :type Boolean) (SweepResult :type Hit%20Result%20Structure%20%28by%20ref%29))
  (if (Actor|ActorHasTag OtherActor "Player")
    (Class|BTSC4|TriggerLineOverlap OtherActor)))

(event EventBeginPlay)

(event Collision|EventActorBeginOverlap
  (params (OtherActor :type Actor%20Object%20Reference)))

(event EventTick
  (params (DeltaSeconds :type Float%20%28single-precision%29)))

(event EventInteractionClear
  (bind _audiocomponent (Variables|Default|GetAudioComponent))
  (|CallParentFunction)
  (Utilities|IsValid _audiocomponent
    (:Is%20Valid
      (Audio|Components|Audio|Stop _audiocomponent))))

(event EventInteraction
  (|CallParentFunction)
  (bind _returnvalue (Audio|SpawnSound2D "/Game/Asset/Sound/UI-Data-Loading-Sound-Effect-_mp3cut_net_.UI-Data-Loading-Sound-Effect-_mp3cut_net_" 1.0 1.0 0.0 0))
  (Variables|Default|SetAudioComponent _returnvalue))

(event EventDestroyed
  (bind _audiocomponent (Variables|Default|GetAudioComponent))
  (Utilities|IsValid _audiocomponent
    (:Is%20Valid
      (Audio|Components|Audio|Stop _audiocomponent))))

(fn ConstructionScript)