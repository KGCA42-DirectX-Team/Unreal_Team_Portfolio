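; BP_C4 is a C4 trap map object that detonates after a character leaves its Line component and can be cleared by interaction.
; End overlap plays delayed repeated shutter sounds, then applies a GameplayEffect to that character with level scaled by distance, spawns particles and destroys itself.
; Interaction shows progress and starts a timer that destroys it without exploding; cancelling pauses the timer.
; The Visible event briefly flashes the clear prompt widget when allowed.
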(event OnComponentEndOverlap(Line)
  (params (OverlappedComponent :type Primitive%20Component%20Object%20Reference) (OtherActor :type Actor%20Object%20Reference) (OtherComp :type Primitive%20Component%20Object%20Reference) (OtherBodyIndex :type Integer))
  (Utilities|ForLoopwithDelay 0 10 0.1
    (:LoopBody
      (Audio|SpawnSoundatLocation "/Engine/VREditor/Sounds/UI/Camera_Shutter.Camera_Shutter" (Transformation|GetWorldLocation OverlappedComponent) "0, 0, 0" 1.0 1.0 0.0 0 0))
    (:Completed
      (bind _asbts_character_base (Utilities|Casting|CastToBTS_CharacterBase OtherActor))
      (GameplayEffects|ApplyGameplayEffectSpecToSelf (Ability|GetAbilitySystemComponent _asbts_character_base) (GameplayEffects|MakeOutgoingSpec :self (Ability|GetAbilitySystemComponent _asbts_character_base) :GameplayEffectClass (Variables|Default|GetGameplay%20Effect%20Class) :Level (/ (Transformation|GetDistanceTo _asbts_character_base self) (Variables|Default|GetExplosionEffectiveDistance))))
      (Effects|SpawnEmitteratLocation "/Engine/Tutorial/SubEditors/TutorialAssets/TutorialParticleSystem.TutorialParticleSystem" (Transformation|GetWorldLocation (Variables|Default|GetC4)))
      (Actor|DestroyActor))))

(event Custom|커스텀이벤트
  (Actor|DestroyActor))

(event EventBeginPlay)

(event Collision|EventActorBeginOverlap
  (params (OtherActor :type Actor%20Object%20Reference)))

(event EventTick
  (params (DeltaSeconds :type Float%20%28single-precision%29)))

(event EventVisible
  (bind _clearwidget (Variables|Default|GetClearWidget))
  (if (Variables|Default|GetWidgetVisible)
    (Rendering|SetVisibility _clearwidget true false)
    (Utilities|FlowControl|Delay 0.1)
    (Rendering|SetVisibility _clearwidget false false)))

(event EventInteraction
  (bind _returnvalue (Utilities|Time|SetTimerbyEvent (delegate Custom|커스텀이벤트) (Variables|Default|GetClearTimer)))
  (Variables|Default|SetTimerHandle _returnvalue)
  (Rendering|SetVisibility (Variables|Default|GetProgress) true false)
  (Variables|Default|SetWidgetVisible false))

(event EventInteractionClaer
  (Utilities|Time|PauseTimerbyHandle (Variables|Default|GetTimerHandle))
  (Variables|Default|SetWidgetVisible true)
  (Rendering|SetVisibility (Variables|Default|GetProgress) false false))

(fn ConstructionScript)