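; BP_HelicopterRope is a map actor, named for a helicopter rope, that reacts when a BP_CinematicPlayer enters its Sphere trigger.
; On overlap it switches the player's movement to Flying and plays the ALS 2m mantle montage on the player's mesh.
; When the montage completes, it applies one large force pushing the player away from the actor and upward.
; The movement mode is not restored here.
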(event OnComponentBeginOverlap(Sphere)
  (params (OverlappedComponent :type Primitive%20Component%20Object%20Reference) (OtherActor :type Actor%20Object%20Reference) (OtherComp :type Primitive%20Component%20Object%20Reference) (OtherBodyIndex :type Integer) (bFromSweep :type Boolean) (SweepResult :type Hit%20Result%20Structure%20%28by%20ref%29))
  (bind _asbp_cinematic_player (Utilities|Casting|CastToBP_CinematicPlayer OtherActor))
  (Pawn|Components|CharacterMovement|SetMovementMode (Variables|/Script/Engine.Character|GetCharacterMovement _asbp_cinematic_player) "MOVE_Flying" 0)
  (Animation|Montage|PlayMontage (Variables|/Script/Engine.Character|GetMesh _asbp_cinematic_player) "/Game/Asset/Animation/UE5Anim/Parkour/AM/ALS_N_Mantle_2m_Montage.ALS_N_Mantle_2m_Montage"
    (:OnCompleted
      (Physics|AddForce (Variables|/Script/Engine.Character|GetCharacterMovement _asbp_cinematic_player) (* (+ (Math|Vector|GetUnitDirection(Vector) (Transformation|GetActorLocation) (Transformation|GetActorLocation _asbp_cinematic_player)) (Transformation|GetActorUpVector _asbp_cinematic_player)) 2.5002e+06)))))

(event EventBeginPlay)

(event Collision|EventActorBeginOverlap
  (params (OtherActor :type Actor%20Object%20Reference)))

(event EventTick
  (params (DeltaSeconds :type Float%20%28single-precision%29)))

(fn ConstructionScript)